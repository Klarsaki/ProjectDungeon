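; Base status effect package holding a buff or debuff's name, priority, tag, source, owner, values and duration, shared across affected characters.
; Unless duration is manual, it binds to the game state's global status interval, counting down 0.1 per tick and calling an empty per-tick hook for children.
; On expiry it unbinds and removes itself from every tracked character; individual removal is also supported.
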(event `StartBlindingToUpdate`
  (params (Character :type "/Game/System/GameCharacter/Bp_BaseCharacter Object Reference"))
  (bind _currentcharacters (`self.CurrentCharacters`))
  (`KismetArrayLibrary.Array_AddUnique` _currentcharacters Character)
  (bind _asgs_ingame_game_state (`/Game/System/GameCharacter/Bp_BaseCharacter.GiveMeGameState` (`|GetArrayItem` _currentcharacters)))
  (set `self.CountDuration` (`self.Duration`))
  (if (not (`self.MannualDuration`))
    (add `/Game/System/Ingame/GS_IngameGameState.Ed_StatusGlobalInterval` _asgs_ingame_game_state (delegate `CustomEvent`))))

(event `CustomEvent`
  (bind _output_get (set `self.CountDuration` (- (`self.CountDuration`) 0.1)))
  (`self.EachTickUpdate`)
  (if (<= _output_get 0.0)
    (remove `/Game/System/Ingame/GS_IngameGameState.Ed_StatusGlobalInterval` (stale `StartBlindingToUpdate` _asgs_ingame_game_state) (delegate `CustomEvent`))
    (`self.RemoveAll`)))

(event `EachTickUpdate`)

(fn `GetValues`
  (params (AddInformation :type "Actor Object Reference") (AddInformation2 :type "Object Object Reference"))
  (returns (NewParam :type "Float (double-precision)"))
  (return (`self.RawValues`)))

(fn `IndividualRemove`
  (params (Target :type "/Game/System/GameCharacter/Bp_BaseCharacter Object Reference"))
  (`KismetArrayLibrary.Array_RemoveItem` (`self.CurrentCharacters`) Target)
  (`/Game/System/GameCharacter/Bp_BaseCharacter.RemoveStatus` Target self))

(fn `RemoveAll`
  (locals (NewLocalVar :type "Array of /Game/System/GameCharacter/Bp_BaseCharacter Object Reference"))
  (bind _output_get (set `local.NewLocalVar` (`self.CurrentCharacters`)))
  (for _array_element _output_get
    (`/Game/System/GameCharacter/Bp_BaseCharacter.RemoveStatus` _array_element self))
  (`KismetArrayLibrary.Array_Clear` (`self.CurrentCharacters`)))

(fn `SetupPackage`
  (params (StatusName :type String :default "Status?") (Description :type String) (Priority :type Integer :default 1) (Duration :type "Float (double-precision)" :default 1.0) (StatusTag :type "/Game/System/Status/Enum_StatusTag Enum" :default "NewEnumerator0") (SourceEvent :type "Actor Object Reference") (Owner :type "/Game/System/GameCharacter/Bp_BaseCharacter Object Reference") (RawValues :type "Float (double-precision)") (Variation :type Integer) (MannualDuration :type Boolean) (isBuff :type Boolean))
  (set `self.StatusName` StatusName)
  (set `self.Description` Description)
  (`|ExecutionSequence`
    (:`then_0`
      (set `self.Priority` Priority))
    (:`then_1`
      (set `self.Duration` Duration))
    (:`then_2`
      (set `self.StatusTagV2` StatusTag))
    (:`then_3`
      (set `self.SourceEvent` SourceEvent))
    (:`then_4`
      (set `self.Owner` Owner))
    (:`then_5`
      (set `self.RawValues` RawValues))
    (:`then_6`
      (set `self.Variation` Variation))
    (:`then_7`
      (set `self.MannualDuration` MannualDuration))
    (:`then_8`
      (set `self.isBuff` isBuff))
    (:`then_9`
      (return))))