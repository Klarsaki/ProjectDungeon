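; Gas trap actor that releases a one-shot cloud of damage over time when a character or "EnviromentAttack"-tagged actor enters its trigger sphere.
; On authority, the trigger disables its overlap events and reveals GasDOT.
; A looping timer damages characters overlapping GasDOT through an interface message, hitting Player-tagged ones harder.
; After about five seconds the timer is cleared and the gas is hidden again.
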(event `self.Sphere.OnComponentBeginOverlap`
  (params (OverlappedComponent :type "PrimitiveComponent Object Reference") (OtherActor :type "Actor Object Reference") (OtherComp :type "PrimitiveComponent Object Reference") (OtherBodyIndex :type Integer) (bFromSweep :type Boolean) (SweepResult :type "HitResult Structure (by ref)"))
  (`/Engine/EditorBlueprintResources/ActorMacros.Switch Has Authority`
    (:`Authority`
      (if (or (`GameplayStatics.ObjectIsA` OtherActor "/Game/System/GameCharacter/Bp_BaseCharacter.Bp_BaseCharacter_C") (`self.ActorHasTag` OtherActor "EnviromentAttack"))
        (`|ExecutionSequence`
          (:`then_0`
            (set `PrimitiveComponent.bGenerateOverlapEvents` false (`self.Sphere`))
            (`SceneComponent.SetHiddenInGame` (`self.GasDOT`) false false))
          (:`then_1`
            (bind _returnvalue (`KismetSystemLibrary.K2_SetTimerDelegate` (delegate `DealDam,age`) 0.5 true))
            (`KismetSystemLibrary.Delay` 5.1)
            (`KismetSystemLibrary.K2_ClearAndInvalidateTimerHandle` _returnvalue)
            (`self.SetActorTickEnabled` false)
            (`SceneComponent.SetHiddenInGame` (`self.GasDOT`) true false)))))))

(event `DealDam,age`
  (for _array_element (`PrimitiveComponent.GetOverlappingActors` (`self.GasDOT`) "/Game/System/GameCharacter/Bp_BaseCharacter.Bp_BaseCharacter_C")
    (message `/Game/System/GameCharacter/Int_StatusPackage.InterfaceCharacterApplyDamage` _array_element (`KismetMathLibrary.SelectFloat` 10.0 5.0 (`self.ActorHasTag` _array_element "Player")) false self (0.0 0.0 0.0) 0.0)))

(fn `UserConstructionScript`)