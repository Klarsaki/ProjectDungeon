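; Single-use bear trap that roots and damages a playable character who steps into its sphere trigger.
; On authority, the overlap applies a timed root status package through an interface, swaps to the snatched mesh and requests damage.
; Actors tagged EnviromentAttack also spring it, without the mesh swap or effects on the actor.
; Either trigger plays the snap sound, disables collision and destroys the trap after a short delay.
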(event `self.Sphere.OnComponentBeginOverlap`
  (params (OverlappedComponent :type "PrimitiveComponent Object Reference") (OtherActor :type "Actor Object Reference") (OtherComp :type "PrimitiveComponent Object Reference") (OtherBodyIndex :type Integer) (bFromSweep :type Boolean) (SweepResult :type "HitResult Structure (by ref)"))
  (`/Engine/EditorBlueprintResources/ActorMacros.Switch Has Authority`
    (:`Authority`
      (if (`GameplayStatics.ObjectIsA` OtherActor "/Game/System/GameCharacter/Bp_BasePlayableCharacter.Bp_BasePlayableCharacter_C")
        (`|ExecutionSequence`
          (:`then_0`
            (bind _returnvalue (`|GenericCreateObject` "/Game/System/Status/Bp_BaseStatusPackage.Bp_BaseStatusPackage_C"))
            (`/Game/System/Status/Bp_BaseStatusPackage.SetupPackage` _returnvalue "RootTest" "RootTarget" 1 2.0 "NewEnumerator6" self null 0.0 0 false false)
            (message `/Game/System/GameCharacter/Int_StatusPackage.InterfaceApplyStatus` OtherActor _returnvalue)
            (`SceneComponent.SetHiddenInGame` (`self.Cube`) true false)
            (`SceneComponent.SetHiddenInGame` (`self.Snatched`) false false))
          (:`then_1`
            (`/Game/System/GameCharacter/Bp_BaseCharacter.Server_RequestApplyDamage` (cast `/Game/System/GameCharacter/Bp_BaseCharacter` OtherActor :!pure true) 40.0 false self (0.0 0.0 0.0) 0.0)
            (`self.SetActorTickEnabled` false :!label _label)
            (`self.PlaySoundSnatched`)
            (`self.SetActorEnableCollision` false)
            (`KismetSystemLibrary.Delay` 2.0)
            (`self.K2_DestroyActor`)))
        (elif (`self.ActorHasTag` OtherActor "EnviromentAttack")
          (goto _label))))))

(event `PlaySoundSnatched`
  (`GameplayStatics.PlaySoundAtLocation` "/Game/Sound/freesound_community-bear-trap-103800.freesound_community-bear-trap-103800" (`self.K2_GetActorLocation`) (struct) 1.4 1.2 0.15 "/Game/Sound/SA_BasicSetting.SA_BasicSetting" null null null))

(fn `UserConstructionScript`)