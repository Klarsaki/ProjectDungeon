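; Base actor for player skills that binds to an owning player on install and gates casting by action state and mana.
; TryCastSkill checks the owner's action passability, spends the mana cost, then fires a client-cast dispatcher and the client played event, printing debug text on failure.
; The client played event forwards to an empty server played event.
; IsSkillCastable reports whether a valid owner has enough mana.
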(event `OnInstallSetup`
  (params (PlayerOwner :type "/Game/System/GameCharacter/Bp_BasePlayableCharacter Object Reference"))
  (set `self.PlayerOwner` PlayerOwner)
  (`KismetSystemLibrary.PrintString` "SkillSetup" true true (struct :`R` 0.802155 :`G` 1.0 :`A` 1.0) 8.0))

(event `Client_SkillPlayed`
  (`self.Server_SkillPlayed`))

(event `Server_SkillPlayed`)

(fn `IsSkillCastable`
  (returns (NewParam :type Boolean))
  (bind _playerowner (`self.PlayerOwner`))
  (`/Engine/EditorBlueprintResources/StandardMacros.IsValid` _playerowner
    (:`Is Valid`
      (return (>= (`/Game/System/GameCharacter/Bp_BasePlayableCharacter.ManaCurrent` _playerowner) (`self.Cost`))))
    (:`Is Not Valid`
      (return false))))

(fn `TryCastSkill`
  (bind _playerowner (`self.PlayerOwner`))
  (if (`/Game/System/GameCharacter/Bp_BasePlayableCharacter.GetActionPassable` _playerowner (`self.Pass if Walkable`) (`self.SpecialPassCondition`))
    (bind _consumesuccess (`/Game/System/GameCharacter/Bp_BasePlayableCharacter.UpdateMana` _playerowner (* (`self.Cost`) -1.0) false))
    (if _consumesuccess
      (`self.Ed_ClientCasted`)
      (`self.Client_SkillPlayed`)
      (else
        (`KismetSystemLibrary.PrintString` "CastSkillFail _ Nomana")))
    (else
      (`KismetSystemLibrary.PrintString` "CastSkillFail _ onAction"))))

(fn `UserConstructionScript`)