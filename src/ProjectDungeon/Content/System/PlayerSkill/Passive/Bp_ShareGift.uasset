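; Passive skill ShareGift, which shares a character's potion effects with the rest of the playable characters.
; On setup it casts the owner to the base playable character and binds to its potion-used event.
; When a potion is used, every other playable character returned by the helper receives half the value, as HP for healing potions or as mana otherwise.
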(event `self.SetupCharPassive`
  (params (Owner :type "/Game/System/GameCharacter/Bp_BaseCharacter Object Reference"))
  (`parent.SetupCharPassive` Owner)
  (bind _asbp_base_playable_character (cast `/Game/System/GameCharacter/Bp_BasePlayableCharacter` Owner))
  (add `/Game/System/GameCharacter/Bp_BasePlayableCharacter.Ed_PotionUsed` _asbp_base_playable_character (delegate `Ed_PotionUsed_Event`)))

(event `Ed_PotionUsed_Event`
  (params (Ishealing :type Boolean) (val :type "Float (double-precision)"))
  (bind _returnvalue (/ val 2.0))
  (bind _owner (`self.Owner`))
  (bind _outactors (`/Game/System/GameCharacter/Bp_BaseCharacter.helper_GetBasePlayableCharacte` _owner))
  (for _array_element _outactors
    (if (!= _array_element _owner)
      (if Ishealing
        (`/Game/System/GameCharacter/Bp_BaseCharacter.UpdateHp` _array_element _returnvalue)
        (else
          (`/Game/System/GameCharacter/Bp_BasePlayableCharacter.UpdateMana` _array_element _returnvalue false))))))