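; Base character class that handles health, damage, knockback and status effects, with empty hooks for children.
; Status packages are sorted by tag into containers for stun, blind, ensnare, speed and damage modifiers, which drive state flags and scales.
; Server damage applies received modifiers, blocking and a mutable pre-damage object broadcast to listeners before HP drops, honoring non-lethal hits.
; Speed modifiers sum into a cached scale whose RepNotify sets clamped walk speed on authority.
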(event `self.ReceiveBeginPlay`
  (`/Engine/EditorBlueprintResources/ActorMacros.Switch Has Authority`
    (:`Authority`
      (`self.SetupStatusManager`))))

(event `OnHpZero`
  (params (KillerSource :type "Actor Object Reference")))

(event `/Game/System/GameCharacter/Int_StatusPackage.InterfaceCharacterApplyDamage`
  (params (Damage :type "Float (double-precision)") (NonLethal :type Boolean) (Source :type "Actor Object Reference") (ContractVector :type "Vector Structure") (KnockForce :type "Float (double-precision)"))
  (`self.Server_RequestApplyDamage` Damage NonLethal Source ContractVector KnockForce))

(event `Server_RequestApplyDamage`
  (params (Damage :type "Float (double-precision)") (NonLethalHit :type Boolean) (Source :type "Actor Object Reference") (ContractVector :type "Vector Structure") (KnockForce :type "Float (double-precision)"))
  (`self.OnDealDamage` Damage NonLethalHit Source)
  (if (>= KnockForce 10.0)
    (`self.LaunchCharacter` (* (`KismetMathLibrary.Vector_Normal2D` (- (`self.K2_GetActorLocation`) (`KismetMathLibrary.SelectVector` (`self.K2_GetActorLocation` Source) ContractVector (== (`KismetMathLibrary.VSize` ContractVector) 0.0)))) KnockForce) true)))

(event `OnApplyStun`
  (params (SourcePackage :type "/Game/System/Status/Bp_BaseStatusPackage Object Reference")))

(event `OnApplyBlind`
  (params (SourcePackage :type "/Game/System/Status/Bp_BaseStatusPackage Object Reference")))

(event `DebugReport`
  (params (TotalDamageDealt :type "Float (double-precision)"))
  (`KismetSystemLibrary.PrintString` (`KismetStringLibrary.Concat_StrStr` "Damage done : " (`KismetStringLibrary.Conv_DoubleToString` TotalDamageDealt)) true true (struct :`R` 1.0 :`G` 0.028473 :`A` 1.0)))

(event `/Game/System/GameCharacter/Int_StatusPackage.InterfaceApplyStatus`
  (params (Source :type "/Game/System/Status/Bp_BaseStatusPackage Object Reference"))
  (`self.ApplyStatus` Source))

(event `/Game/System/GameCharacter/Int_StatusPackage.InterfaceRemoveStatus`
  (params (SourceTarget :type "/Game/System/Status/Bp_BaseStatusPackage Object Reference"))
  (`self.RemoveStatus` SourceTarget))

(event `WhenMsUpdated`
  (`self.MovementSpeedManager`))

(event `SetupStatusManager`
  (add `self.Ed_MovementSpeedUpdate` (delegate `WhenMsUpdated`))
  (`self.Ed_MovementSpeedUpdate`))

(event `SetMovementSpeedOnClient`
  (params (NewResultScale :type "Float (single-precision)"))
  ; Compute speed and cached
  (set `self.ResultModifiedScaleCachedSpeed` NewResultScale))

(event `LocalSpeedUpdateNoticing`)

(event `SetSpeedOnServer`
  (params (`Max Walk Speed` :type "Float (single-precision)"))
  (set `CharacterMovementComponent.MaxWalkSpeed` `Max Walk Speed` (`self.CharacterMovement`)))

(event `AddStatus_Stun`
  (params (SourcePackage :type "/Game/System/Status/Bp_BaseStatusPackage Object Reference"))
  (`KismetArrayLibrary.Array_AddUnique` (`self.StatusContainer_Stun`) SourcePackage)
  (set `self.isStunning` true)
  (`self.Ed_StatusAdded` SourcePackage)
  (`KismetSystemLibrary.PrintString` "StunComing")
  (`self.OnApplyStun` SourcePackage))

(event `DebugSphere`
  (params (Center :type "Vector Structure") (Radius :type "Float (single-precision)"))
  (`KismetSystemLibrary.DrawDebugSphere` Center Radius 12 (struct :`R` 1.0 :`G` 0.012015 :`A` 1.0) 0.2))

(event `RemovingCheck`
  (if (> (`KismetArrayLibrary.Array_Length` (`self.StatusContainer_Stun`)) 0)
    (set `self.isStunning` true)
    (else
      (set `self.isStunning` false)
      (`KismetSystemLibrary.PrintString` "StunEnd"))))

(event `CreateSimpleClueDrop`
  (params (CreatePosition :type "Vector Structure") (Radius :type "Float (double-precision)") (AlertPosition :type "Vector Structure") (Agroyer :type "/Game/System/GameCharacter/Bp_BasePlayableCharacter Object Reference") (AgroRate :type "Float (double-precision)") (ActorsToIgnore :type "Array of Actor Object Reference (by ref)"))
  (bind _outactors (`KismetSystemLibrary.SphereOverlapActors` CreatePosition Radius (`|MakeArray` "ObjectTypeQuery3" :!type "EObjectTypeQuery Enum") "/Game/System/GameCharacter/Enemies/Bp_BaseEnemy.Bp_BaseEnemy_C" ActorsToIgnore))
  (for _array_element _outactors
    (message `/Game/System/GameCharacter/Enemies/INT_BpEnemy.CluedropToEnemy` _array_element AlertPosition Agroyer AgroRate)))

(event `AddStatus_Blind`
  (params (SourcePackage :type "/Game/System/Status/Bp_BaseStatusPackage Object Reference"))
  (`KismetArrayLibrary.Array_AddUnique` (`self.StatusContainer_Blind`) SourcePackage)
  (set `self.isBlinding` true)
  (`self.Ed_StatusAdded` SourcePackage)
  (`KismetSystemLibrary.PrintString` "Bindcome")
  (`self.OnApplyBlind` SourcePackage))

(event `BlindRemoveCheck`
  (if (> (`KismetArrayLibrary.Array_Length` (`self.StatusContainer_Blind`)) 0)
    (set `self.isBlinding` true)
    (else
      (set `self.isBlinding` false)
      (`KismetSystemLibrary.PrintString` "BlindEnd"))))

(event `AddStatus_Ensnare`
  (params (SourcePackage :type "/Game/System/Status/Bp_BaseStatusPackage Object Reference (by ref)"))
  (`KismetArrayLibrary.Array_AddUnique` (`self.StatusContainer_Ensnare`) SourcePackage)
  (set `self.Ensnared` true)
  (`self.AsEnsared`)
  (`self.Ed_StatusAdded` SourcePackage))

(event `OnEnsnare`)

(event `RemoveEnsnareCheck`
  (if (not (> (`KismetArrayLibrary.Array_Length` (`self.StatusContainer_Ensnare`)) 0))
    (set `self.Ensnared` false)
    (`self.AsEnsared`)
    (`KismetSystemLibrary.PrintString` "EnsnareEnd")))

(event `AddStatus_MoveSpeedMod`
  (params (SourcePackage :type "/Game/System/Status/Bp_BaseStatusPackage Object Reference"))
  (`KismetArrayLibrary.Array_AddUnique` (`self.StatusContainer_MovementSpeedMod`) SourcePackage)
  (`self.Ed_StatusAdded` SourcePackage)
  (`self.Ed_MovementSpeedUpdate`))

(event `AddStatus_DamageDealtMod`
  (params (SourcePackage :type "/Game/System/Status/Bp_BaseStatusPackage Object Reference (by ref)"))
  (`KismetArrayLibrary.Array_AddUnique` (`self.StatusContainer_DamageDealt`) SourcePackage)
  (`self.Ed_StatusAdded` SourcePackage))

(event `AddStatus_DamageRecieveMod`
  (params (SourcePackage :type "/Game/System/Status/Bp_BaseStatusPackage Object Reference (by ref)"))
  (`KismetArrayLibrary.Array_AddUnique` (`self.StatusContainer_DamageRecieveMod`) SourcePackage)
  (`self.Ed_StatusAdded` SourcePackage))

(fn `ApplyStatus`
  (params (SourcePackage :type "/Game/System/Status/Bp_BaseStatusPackage Object Reference"))
  (`|ExecutionSequence`
    (:`then_0`
      (switch `/Game/System/Status/Enum_StatusTag` (`/Game/System/Status/Bp_BaseStatusPackage.StatusTagV2` SourcePackage)
        (:`NewEnumerator0`
          (`self.AddStatus_Stun` SourcePackage))
        (:`NewEnumerator1`
          (`self.AddStatus_Blind` SourcePackage))
        (:`NewEnumerator2`
          (`self.AddStatus_MoveSpeedMod` SourcePackage))
        (:`NewEnumerator3`
          (`self.AddStatus_DamageDealtMod` SourcePackage))
        (:`NewEnumerator4`
          (`self.AddStatus_DamageRecieveMod` (`local.SourcePackage`)))
        (:`NewEnumerator6`
          (`self.AddStatus_Ensnare` (`local.SourcePackage`)))))
    (:`then_1`
      (`/Game/System/Status/Bp_BaseStatusPackage.StartBlindingToUpdate` (`local.SourcePackage`) self))))

(fn `AsEnsared`
  (`/Engine/EditorBlueprintResources/ActorMacros.Switch Has Authority`
    (:`Authority`
      (`self.OnEnsnare`))))

(fn `CallDamageModifierPackage`
  (params (InDamage :type "Float (double-precision)"))
  (returns (OutDamage :type "Float (double-precision)"))
  (return 0.0))

(fn `DamageCalculator`
  (params (BaseDamage :type "Float (double-precision)") (AddInformation :type "Actor Object Reference") (AddInformation2 :type "Object Object Reference"))
  (returns (OutputDamage :type "Float (double-precision)"))
  (locals (ScaleDmg :type "Float (double-precision)" :default 1.0))
  (for _array_element (`self.StatusContainer_DamageDealt`)
    (bind _newparam (`/Game/System/Status/Bp_BaseStatusPackage.GetValues` _array_element AddInformation AddInformation2))
    (set `local.ScaleDmg` (+ (`local.ScaleDmg`) _newparam)))
  (return (* (`local.BaseDamage`) (`local.ScaleDmg`))))

(fn `GetBasicWalkSpeed`
  (returns (ReturnValue :type "Float (double-precision)"))
  (return (`KismetMathLibrary.SelectFloat` (`self.MovespeedSprint`) (`self.MovespeedNormal`) (`self.isSprinting`))))

(fn `GiveMeGameState`
  (returns (`AsGS Ingame Game State` :type "/Game/System/Ingame/GS_IngameGameState Object Reference"))
  (bind _asgs_ingame_game_state (cast `/Game/System/Ingame/GS_IngameGameState` (`GameplayStatics.GetGameState`)))
  (return _asgs_ingame_game_state))

(fn `MovementSpeedManager`
  (locals (CacheSpeed :type "Float (double-precision)"))
  (for _array_element (`self.StatusContainer_MovementSpeedMod`)
    (bind _newparam (`/Game/System/Status/Bp_BaseStatusPackage.GetValues` _array_element null null))
    (set `local.CacheSpeed` (+ (`local.CacheSpeed`) _newparam)))
  (`self.SetMovementSpeedOnClient` (+ 1.0 (`local.CacheSpeed`))))

(fn `OnDealDamage`
  (params (TotalDamage :type "Float (double-precision)") (NonLethal :type Boolean :default false) (Source :type "Actor Object Reference"))
  (locals (LocalStashedDamage :type "Float (double-precision)") (LocalInformationHolder :type "/Game/System/GameCharacter/PreRecievDamageRef Object Reference") (BeforeHp :type "Float (double-precision)" :default 0.0) (DamageScale :type "Float (double-precision)" :default 1.0))
  (bind _localinformationholder (`local.LocalInformationHolder`))
  (bind _hpcurrent (`self.HpCurrent`))
  (set `local.LocalStashedDamage` TotalDamage)
  (set `local.BeforeHp` (`self.HpCurrent`))
  (`|ExecutionSequence`
    (:`then_0`
      (for _array_element (`self.StatusContainer_DamageRecieveMod`)
        (bind _newparam (`/Game/System/Status/Bp_BaseStatusPackage.GetValues` _array_element self null)) ; AddInformation = target return in percentile
        (set `local.DamageScale` (+ (`local.DamageScale`) _newparam)))
      (set `local.LocalStashedDamage` (* (`local.LocalStashedDamage`) (`KismetMathLibrary.FClamp` (`local.DamageScale`) 0.0 9999.0))))
    (:`then_1`
      (if (`self.isBlocking`)
        (`self.Ed_DamageBlock` (`local.LocalStashedDamage`))
        (set `local.LocalStashedDamage` 0.0)
        (`KismetSystemLibrary.PrintString` "Blocked")))
    (:`then_2`
      (bind _returnvalue (`|GenericCreateObject` "/Game/System/GameCharacter/PreRecievDamageRef.PreRecievDamageRef_C"))
      (bind _output_get (set `local.LocalInformationHolder` _returnvalue))
      (`/Game/System/GameCharacter/PreRecievDamageRef.SetupPackage` _output_get (`local.LocalStashedDamage`) (`self.Non Lethal`) (`local.Source`))
      (`self.Ed_PreRecieveDamage` (`local.LocalInformationHolder`))
      (`self.UpdateHp` (* (`/Game/System/GameCharacter/PreRecievDamageRef.TotalDamage` _localinformationholder) -1.0))
      (if (`/Game/System/GameCharacter/PreRecievDamageRef.Nonlethal` _localinformationholder)
        (set `self.HpCurrent` (`KismetMathLibrary.FClamp` _hpcurrent 1.0 (`self.HpMax`)))
        (elif (<= _hpcurrent 0.0)
          (`self.OnHpZero` (`local.Source`)))))
    (:`then_3`
      (`self.Ed_PostRecievDamage` (- (`local.BeforeHp`) (`self.HpCurrent`)) Source))
    (:`then_4`
      ; Debug damage source report
      (bind _asbp_base_weapon_class (cast `/Game/System/WeaponClass/Bp_BaseWeaponClass` Source)
        (:`then`
          (`self.DebugReport` (`/Game/System/WeaponClass/Bp_BaseWeaponClass.Holder` _asbp_base_weapon_class) (- (`local.BeforeHp`) (`self.HpCurrent`))))
        (:`CastFailed`
          (bind _asbp_base_skill (cast `/Game/System/PlayerSkill/Bp_BaseSkill` Source))
          (`self.DebugReport` (`/Game/System/PlayerSkill/Bp_BaseSkill.PlayerOwner` _asbp_base_skill) (- (`local.BeforeHp`) (`self.HpCurrent`))))))))

(fn `OnRep_isBlinding`
  (`/Engine/EditorBlueprintResources/ActorMacros.Switch Has Authority`
    (:`Authority`
      (`self.Ed_BlindUpdate`))))

(fn `OnRep_isSprinting`
  (`self.SprintIsUpdate`))

(fn `OnRep_isStunning`
  (`/Engine/EditorBlueprintResources/ActorMacros.Switch Has Authority`
    (:`Authority`
      (`self.Ed_StunUpdate`))))

(fn `OnRep_ResultModifiedScaleCachedSpeed`
  (`/Engine/EditorBlueprintResources/ActorMacros.Switch Has Authority`
    (:`Authority`
      (`self.SetSpeedOnServer` (`KismetMathLibrary.FClamp` (* (`self.GetBasicWalkSpeed`) (`self.ResultModifiedScaleCachedSpeed`)) 80.0 9999.0)))
    (:`Remote`
      (`self.LocalSpeedUpdateNoticing`))))

(fn `RemoveStatus`
  (params (TargetStatus :type "/Game/System/Status/Bp_BaseStatusPackage Object Reference"))
  (locals (NewLocalVar :type "/Game/System/Status/Bp_BaseStatusPackage Object Reference"))
  (bind _output_get (set `local.NewLocalVar` TargetStatus))
  (`/Engine/EditorBlueprintResources/ActorMacros.Switch Has Authority`
    (:`Authority`
      (switch `/Game/System/Status/Enum_StatusTag` (`/Game/System/Status/Bp_BaseStatusPackage.StatusTagV2` _output_get)
        (:`NewEnumerator0`
          (`KismetArrayLibrary.Array_RemoveItem` (`self.StatusContainer_Stun`) _output_get)
          (`self.RemovingCheck`))
        (:`NewEnumerator1`
          (`KismetArrayLibrary.Array_RemoveItem` (`self.StatusContainer_Blind`) _output_get)
          (`self.BlindRemoveCheck`))
        (:`NewEnumerator2`
          (`KismetArrayLibrary.Array_RemoveItem` (`self.StatusContainer_MovementSpeedMod`) (`local.NewLocalVar`))
          (`self.Ed_MovementSpeedUpdate`))
        (:`NewEnumerator3`
          (`KismetArrayLibrary.Array_RemoveItem` (`self.StatusContainer_DamageDealt`) (`local.NewLocalVar`)))
        (:`NewEnumerator4`
          (`KismetArrayLibrary.Array_RemoveItem` (`self.StatusContainer_DamageRecieveMod`) (`local.NewLocalVar`)))
        (:`NewEnumerator6`
          (`KismetArrayLibrary.Array_RemoveItem` (`self.StatusContainer_Ensnare`) (`local.NewLocalVar`))
          (`self.RemoveEnsnareCheck`))))))

(fn `SprintIsUpdate`)

(fn `UpdateHp`
  (params (IncomingVal :type "Float (double-precision)"))
  (set `self.HpCurrent` (`KismetMathLibrary.FClamp` (+ (`self.HpCurrent`) IncomingVal) 0.0 (`self.HpMax`))))

(fn `UserConstructionScript`)