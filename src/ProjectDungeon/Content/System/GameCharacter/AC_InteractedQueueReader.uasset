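; Actor component on the playable character that queues nearby interactables and requests interaction with a chosen target.
; Add and remove functions maintain AllInteractable, inserting newcomers at the front; type-based ordering is disconnected.
; GetObjectToInteraction stores the object best aligned with control rotation, using a dot product above 0.5.
; TryInteractToCurrentTarget passes that target through ServerRequestInteract to AsInteracted; automatic target refresh is unwired here.
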(event `self.ReceiveBeginPlay`
  (bind _asbp_base_playable_character (cast `/Game/System/GameCharacter/Bp_BasePlayableCharacter` (`self.GetOwner`)))
  (set `self.As Bp Base Playable Character` _asbp_base_playable_character))

(event `IniSetup`)

(event `self.ReceiveTick`
  (params (DeltaSeconds :type "Float (single-precision)")))

(event `ServerRequestInteract`
  (params (Target :type "/Game/System/InteractSystem/Bp_InteractableObject Object Reference"))
  (`/Game/System/InteractSystem/Bp_InteractableObject.AsInteracted` Target self))

(event `TryInteractToCurrentTarget`
  (`self.ServerRequestInteract` (`self.ShouldInteracted`)))

(fn `AddIncomingInteractable`
  (params (NewObject :type "/Game/System/InteractSystem/Bp_InteractableObject Object Reference"))
  (locals (`isAdded?` :type Boolean))
  (`KismetSystemLibrary.PrintString` "Add interaction to only local screen")
  (`KismetArrayLibrary.Array_Insert` (`self.AllInteractable`) NewObject))

(fn `GetObjectToInteraction`
  (returns (NewParam :type "/Game/System/InteractSystem/Bp_InteractableObject Object Reference"))
  (locals (SetKeepable :type "/Game/System/InteractSystem/Bp_InteractableObject Object Reference") (CurrentDot :type "Float (double-precision)" :default 0.0))
  (bind _as_bp_base_playable_character (`self.As Bp Base Playable Character`))
  (for _array_element (`self.AllInteractable`)
    (bind _returnvalue (`KismetMathLibrary.Dot_VectorVector` (`KismetMathLibrary.GetForwardVector` (`Pawn.GetControlRotation` _as_bp_base_playable_character)) (`KismetMathLibrary.Normal` (- (`Actor.K2_GetActorLocation` _array_element) (`Actor.K2_GetActorLocation` _as_bp_base_playable_character)))))
    (if (> _returnvalue 0.5)
      (`/Engine/EditorBlueprintResources/StandardMacros.IsValid` (`local.SetKeepable`)
        (:`Is Valid`
          (if (> _returnvalue (`local.CurrentDot`))
            (set `local.CurrentDot` _returnvalue)
            (set `local.SetKeepable` _array_element)))
        (:`Is Not Valid`
          (set `local.CurrentDot` _returnvalue)
          (set `local.SetKeepable` _array_element)))))
  (bind _output_get (set `self.ShouldInteracted` (`local.SetKeepable`)))
  (return _output_get))

(fn `RemoveInteractable`
  (params (NewObject :type "/Game/System/InteractSystem/Bp_InteractableObject Object Reference"))
  (returns (`Success?` :type Boolean))
  (locals (`isAdded?` :type Boolean))
  (bind _returnvalue (`KismetArrayLibrary.Array_RemoveItem` (`self.AllInteractable`) NewObject))
  (return _returnvalue))