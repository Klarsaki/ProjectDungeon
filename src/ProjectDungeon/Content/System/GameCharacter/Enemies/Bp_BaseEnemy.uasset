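; Base enemy character that runs a StateTree AI, started with an area manager that relays group alerts when it acquires a target.
; Server-side logic picks actions by chance-weighted random from range and line-of-sight checks, and defers queued target changes until actions end.
; Blind, stun and charm interrupt or redirect it, while helpers rotate it toward targets.
; Death stops AI, drops an alert clue and enables an overlap sphere granting items, previewed as attached meshes.
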(event `self.OnHpZero`
  (params (KillerSource :type "Actor Object Reference"))
  (if (not (`self.isDead`))
    (`|ExecutionSequence`
      (:`then_0`
        (set `self.isDead` true)
        (`self.Ed_DeathCall`)
        (set `self.Killer Source` KillerSource))
      (:`then_1`
        (bind _asbp_base_character (cast `/Game/System/GameCharacter/Bp_BaseCharacter` (`self.GetOwner` KillerSource)))
        (`self.TryGetKiller` _asbp_base_character))
      (:`then_2`
        (`BrainComponent.StopLogic` (`self.StateTree`) "Target dead")
        (`self.AsDeath`)))))

(event `TryGetKiller`
  (params (Target :type "/Game/System/GameCharacter/Bp_BaseCharacter Object Reference"))
  (`self.Ed_ActorJustKillTarget` Target (stale `self.OnHpZero` KillerSource))
  (bind _asbp_base_playable_character (cast `/Game/System/GameCharacter/Bp_BasePlayableCharacter` Target))
  (`self.CreateSimpleClueDrop` (`self.K2_GetActorLocation`) 800.0 (`self.K2_GetActorLocation` Target) _asbp_base_playable_character 0.2))

(event `AsDeath`
  (`|PlayMontage` (`self.Mesh`) "/Game/Characters/Mannequins/Anims/Death/MM_Death_Front_02_Montage.MM_Death_Front_02_Montage"
    (:`then`
      (`|ExecutionSequence`
        (:`then_0`
          (`PrimitiveComponent.SetCollisionEnabled` (`self.CapsuleComponent`) "NoCollision")
          (`CharacterMovementComponent.DisableMovement` (`self.CharacterMovement`))
          (`KismetSystemLibrary.Delay` 2.0)
          (`self.SetActorHiddenInGame` true))
        (:`then_1`
          (`/Engine/EditorBlueprintResources/ActorMacros.Switch Has Authority`
            (:`Authority`
              (`self.DeathDrop`))))))))

(event `AddItemToTarget`
  (params (Target :type "/Game/System/GameCharacter/Bp_BasePlayableCharacter Object Reference"))
  (for _array_element (`self.DropingItem`)
    (`/Game/System/Ingame/Inventory/Bp_InventoryHolder.AddItemToInventory` (`/Game/System/GameCharacter/Bp_BasePlayableCharacter.Bp_InventoryHolder` Target) (break `/Game/System/Item/Struct_EnemyItemDrop` _array_element) (`.Amount_7_4ED2B962470779D271CC69B3FB3330A3` (break `/Game/System/Item/Struct_EnemyItemDrop` _array_element)))
    (`KismetSystemLibrary.PrintString` "KeyAdded"))
  (set `PrimitiveComponent.bGenerateOverlapEvents` false (`self.Sphere`)))

(event `DeathDrop`
  (set `PrimitiveComponent.bGenerateOverlapEvents` true (`self.Sphere`)))

(event `self.Sphere.OnComponentBeginOverlap`
  (params (OverlappedComponent :type "PrimitiveComponent Object Reference") (OtherActor :type "Actor Object Reference") (OtherComp :type "PrimitiveComponent Object Reference") (OtherBodyIndex :type Integer) (bFromSweep :type Boolean) (SweepResult :type "HitResult Structure (by ref)"))
  (bind _asbp_base_playable_character (cast `/Game/System/GameCharacter/Bp_BasePlayableCharacter` OtherActor))
  (`self.AddItemToTarget` _asbp_base_playable_character))

(event `LooktoLocation`
  (params (TargetLo :type "Vector Structure") (GoalDotAngle :type "Float (double-precision)" :default 0.7))
  (bind (_returnvalue_roll _returnvalue_pitch) (`KismetMathLibrary.BreakRotator` (`self.K2_GetActorRotation`)))
  (bind _pawnsensing (`self.PawnSensing`))
  (bind (_returnvalue_roll_2 _returnvalue_pitch_2 _returnvalue_yaw) (`KismetMathLibrary.BreakRotator` (`KismetMathLibrary.FindLookAtRotation` (`self.K2_GetActorLocation`) TargetLo)))
  (bind (_returnvalue_roll_3 _returnvalue_pitch_3 _returnvalue_yaw_2) (`KismetMathLibrary.BreakRotator` (`KismetMathLibrary.RInterpTo` (`self.K2_GetActorRotation`) (`KismetMathLibrary.MakeRotator` 0.0 0.0 _returnvalue_yaw) (`GameplayStatics.GetWorldDeltaSeconds`) 4.0)))
  (add `self.Ed_Interupted` (delegate `Interupter`))
  (`|ExecutionSequence`
    (:`then_0`
      (goto _label_2 :!via `Reset`))
    (:`then_1`
      (`Timeline|LookToTimeliner` :!via `PlayFromStart` :!label _label
        (:`Update`
          (`self.K2_SetActorRotation` (`KismetMathLibrary.MakeRotator` _returnvalue_roll _returnvalue_pitch _returnvalue_yaw_2))
          (`|ExecutionSequence`
            (:`then_0`
              (if (> (`KismetMathLibrary.VSize` (`MovementComponent.Velocity` (`self.CharacterMovement`))) 1.0)
                (`TimelineComponent.Stop` (`self.LookToTimeliner`))))
            (:`then_1`
              (if (> (`KismetMathLibrary.Dot_VectorVector` (`self.GetActorForwardVector`) (`KismetMathLibrary.Vector_Normal2D` (- TargetLo (`self.K2_GetActorLocation`)))) GoalDotAngle)
                (`/Engine/EditorBlueprintResources/StandardMacros.DoOnce` false :!label _label_2
                  (:`Completed`
                    (remove `self.Ed_Interupted` (delegate `Interupter`))
                    (`PawnSensingComponent.SetSensingUpdatesEnabled` _pawnsensing false)
                    (`PawnSensingComponent.SetSensingUpdatesEnabled` _pawnsensing true)
                    (`self.Ed_ActionEnd` "Rotate")
                    (`KismetSystemLibrary.PrintString` "SuccessRotate")))))))
        (:`Finished`
          (`KismetSystemLibrary.PrintString` "FailToFinishRotate")
          (goto _label_2))))))

(event `self.ReceiveBeginPlay`
  (`parent.ReceiveBeginPlay`)
  (`/Engine/EditorBlueprintResources/ActorMacros.Switch Has Authority`
    (:`Authority`
      (`|ExecutionSequence`
        (:`then_0`
          (if (`self.RoamAsArea`)
            (`KismetArrayLibrary.Array_Set` (`self.RoamPositions`) 0 (`self.K2_GetActorLocation`) true)))))))

(event `Interupter`
  (goto _label :!via `Stop`))

(event `StartupAi`
  (params (AreaManager :type "/Game/System/GameCharacter/Enemies/Bp_AreaEnemiesManager Object Reference"))
  (`/Engine/EditorBlueprintResources/StandardMacros.DoOnce` false
    (:`Completed`
      (set `self.AreaManager` AreaManager)
      (`BrainComponent.StartLogic` (`self.StateTree`)) ; RunOnlyOnServer
      (add `self.Ed_Interupted` (delegate `CustomEvent_0`)))))

(event `self.ReceiveTick`
  (params (DeltaSeconds :type "Float (single-precision)"))
  (`parent.ReceiveTick` DeltaSeconds)
  (`self.KeepRotation`))

(event `CustomEvent_0`
  (set `self.IsOnAction` false))

(event `KeepRotation`
  (bind _currenttarget (`self.CurrentTarget`))
  (bind (_returnvalue_roll _returnvalue_pitch _returnvalue_yaw) (`KismetMathLibrary.BreakRotator` (`KismetMathLibrary.FindLookAtRotation` (`self.K2_GetActorLocation`) (`self.K2_GetActorLocation` _currenttarget))))
  (`/Engine/EditorBlueprintResources/StandardMacros.IsValid` _currenttarget
    (:`Is Valid`
      (if (`self.RotateToCurrentTarget`)
        (`self.K2_SetActorRotation` (`KismetMathLibrary.RInterpTo` (`self.K2_GetActorRotation`) (`KismetMathLibrary.MakeRotator` 0.0 0.0 _returnvalue_yaw) (`GameplayStatics.GetWorldDeltaSeconds`) 6.0))))))

(event `AfterRandomed`
  (params (Selection :type String)))

(event `TryAlert`
  (params (AlertPosition :type "Vector Structure") (Agroyer :type "/Game/System/GameCharacter/Bp_BasePlayableCharacter Object Reference"))
  (bind _areamanager (`self.AreaManager`))
  (`/Engine/EditorBlueprintResources/ActorMacros.Switch Has Authority`
    (:`Authority`
      (`/Engine/EditorBlueprintResources/StandardMacros.IsValid` _areamanager
        (:`Is Valid`
          (`/Game/System/GameCharacter/Enemies/Bp_AreaEnemiesManager.GroupAlert` _areamanager AlertPosition Agroyer))))))

(event `Set Current Target`
  (params (CurrentTarget :type "/Game/System/GameCharacter/Bp_BasePlayableCharacter Object Reference"))
  ; Set current target
  (bind _output_get (set `self.CurrentTarget` CurrentTarget))
  (`self.Ed_SetATarget` _output_get)
  (`/Engine/EditorBlueprintResources/StandardMacros.IsValid` _output_get
    (:`Is Valid`
      (`self.TryAlert` (`self.K2_GetActorLocation` _output_get) _output_get)
      (set `self.ChangingTargetOncooldown` true)
      (`KismetSystemLibrary.RetriggerableDelay` (`KismetMathLibrary.SelectFloat` 5.0 0.1 (`KismetSystemLibrary.IsValid` _output_get)))
      (set `self.ChangingTargetOncooldown` false))))

(event `ActionCall`
  ; Comment
  (`/Engine/EditorBlueprintResources/ActorMacros.Switch Has Authority`
    (:`Authority`
      (bind _resultaction (`self.RandomizeAction`))
      (`self.AfterRandomed` _resultaction))))

(event `OnAlert`
  (params (AlertPosition :type "Vector Structure") (Agroyer :type "/Game/System/GameCharacter/Bp_BasePlayableCharacter Object Reference"))
  (`self.Ed_ClueDrop` AlertPosition Agroyer 0.2))

(event `QueueChangeTarget`
  (params (NextTarget :type "/Game/System/GameCharacter/Bp_BasePlayableCharacter Object Reference"))
  ; Queue set current target -- dont change if on action
  (`/Engine/EditorBlueprintResources/ActorMacros.Switch Has Authority`
    (:`Authority`
      (remove `self.Ed_ActionStateChange` (delegate `CustomEvent_2`))
      (if (`self.IsOnAction`)
        (add `self.Ed_ActionStateChange` (delegate `CustomEvent_2`))
        (else
          (`self.Set Current Target` NextTarget))))))

(event `/Game/System/GameCharacter/Enemies/INT_BpEnemy.CluedropToEnemy`
  (params (AgroPos :type "Vector Structure") (Agroyer :type "/Game/System/GameCharacter/Bp_BasePlayableCharacter Object Reference") (Rate :type "Float (double-precision)"))
  (`self.ClueDropFromAction` AgroPos Agroyer Rate))

(event `ClueDropFromAction`
  (params (AlertPosition :type "Vector Structure") (Agroyer :type "/Game/System/GameCharacter/Bp_BasePlayableCharacter Object Reference") (AgroRate :type "Float (double-precision)"))
  (`self.Ed_ClueDrop` AlertPosition Agroyer AgroRate))

(event `CustomEvent_2`
  ; Queue set current target -- dont change if on action
  (if (not (`self.IsOnAction`))
    (remove `self.Ed_ActionStateChange` (delegate `CustomEvent_2`))
    (`self.Set Current Target` (stale `QueueChangeTarget` NextTarget))))

(event `RefreshAgroCountTimer`
  (bind _returnvalue (`KismetSystemLibrary.K2_SetTimerDelegate` (delegate `CustomEvent`) 15.0))
  (set `self.AgroTimer` _returnvalue))

(event `TryNewAggro`
  (params (Player :type "/Game/System/GameCharacter/Bp_BasePlayableCharacter Object Reference") (AggroRate :type "Float (double-precision)"))
  (`self.Ed_NewAggro` Player AggroRate))

(event `CustomEvent`)

(event `self.Server_RequestApplyDamage`
  (params (Damage :type "Float (double-precision)") (NonLethalHit :type Boolean) (Source :type "Actor Object Reference") (ContractVector :type "Vector Structure") (KnockForce :type "Float (double-precision)"))
  (`parent.Server_RequestApplyDamage` Damage NonLethalHit Source ContractVector KnockForce))

(event `PlayBlind`
  (bind _returnvalue (`SkeletalMeshComponent.GetAnimInstance` (`self.Mesh`)))
  (if (not (== (`AnimInstance.GetCurrentActiveMontage` _returnvalue) (`self.DefaultOnStunMontage`)))
    (`AnimInstance.Montage_Stop` _returnvalue 0.0 null)))

(event `self.OnApplyBlind`
  (params (SourcePackage :type "/Game/System/Status/Bp_BaseStatusPackage Object Reference"))
  (`/Engine/EditorBlueprintResources/ActorMacros.Switch Has Authority`
    (:`Authority`
      (`self.Ed_Interupted`)
      (`self.PlayBlind`)
      (`self.Set Current Target` null))))

(event `self.OnApplyStun`
  (params (SourcePackage :type "/Game/System/Status/Bp_BaseStatusPackage Object Reference"))
  (`/Engine/EditorBlueprintResources/ActorMacros.Switch Has Authority`
    (:`Authority`
      (`self.Ed_Interupted`)
      (`self.PlayStunAnim`))))

(event `PlayStunAnim`
  (`|PlayMontage` (`self.Mesh`) (`self.DefaultOnStunMontage`)))

(event `IfInterupted`
  (`/Engine/EditorBlueprintResources/StandardMacros.IsValid` (`self.LastestCharm`)
    (:`Is Valid`
      (`self.RemoveStatus` (`self.LastestCharm`)))
    (:`Is Not Valid`
      (remove `self.Ed_Interupted` (delegate `IfInterupted`)))))

(event `OnApplyCharm`
  (params (SourcePackage :type "/Game/System/Status/Bp_BaseStatusPackage Object Reference"))
  (bind _owner (`/Game/System/Status/Bp_BaseStatusPackage.Owner` SourcePackage))
  (`/Engine/EditorBlueprintResources/ActorMacros.Switch Has Authority`
    (:`Authority`
      (set `self.LastestCharm` SourcePackage)
      (add `self.Ed_Interupted` (delegate `IfInterupted`))
      (bind _output_get (set `self.LastestAggroyer` (cast `/Game/System/GameCharacter/Bp_BasePlayableCharacter` _owner :!pure true)))
      (set `self.LastestReadClue` (`self.K2_GetActorLocation` _owner))
      (`self.Ed_CharmApplyed`)
      (if (not (`self.IsOnAction`))
        (`self.Set Current Target` _output_get)))))

(fn `ApplyStatus`
  (params (SourcePackage :type "/Game/System/Status/Bp_BaseStatusPackage Object Reference"))
  (`|ExecutionSequence`
    (:`then_0`
      (switch `/Game/System/Status/Enum_StatusTag` (`/Game/System/Status/Bp_BaseStatusPackage.StatusTagV2` SourcePackage)
        (:`NewEnumerator5`
          (`self.OnApplyCharm` SourcePackage))))
    (:`then_1`
      (`parent.ApplyStatus` SourcePackage))))

(fn `Get Current Target`
  (returns (CurrentTarget :type "/Game/System/GameCharacter/Bp_BasePlayableCharacter Object Reference"))
  (return (`self.CurrentTarget`)))

(fn `OnRep_IsOnAction`
  (bind _lastestcharm (`self.LastestCharm`))
  (`/Engine/EditorBlueprintResources/ActorMacros.Switch Has Authority`
    (:`Authority`
      (`self.Ed_ActionStateChange`)
      (if (not (`self.IsOnAction`))
        (`|ExecutionSequence`
          (:`then_0`
            (`/Engine/EditorBlueprintResources/StandardMacros.IsValid` _lastestcharm
              (:`Is Valid`
                (`self.Set Current Target` (cast `/Game/System/GameCharacter/Bp_BasePlayableCharacter` (`/Game/System/Status/Bp_BaseStatusPackage.Owner` _lastestcharm) :!pure true))))))))))

(fn `OnRep_LastestAggroyer`
  (`/Engine/EditorBlueprintResources/ActorMacros.Switch Has Authority`
    (:`Authority`
      (`self.RefreshAgroCountTimer`))))

(fn `RandomizeAction`
  (returns (ResultAction :type String))
  (locals (SavedString :type "Array of String") (FinalResult :type String) (SeePlayer :type Boolean) (CachePlayers :type "Array of /Game/System/GameCharacter/Bp_BasePlayableCharacter Object Reference"))
  (bind _lockaction (`self.LockAction`))
  (bind _returnvalue (`self.GetDistanceTo` self (`self.CurrentTarget`)))
  (if (== _lockaction "")
    (`|ExecutionSequence`
      (:`then_0`
        (bind (_outhit _returnvalue_2) (`KismetSystemLibrary.LineTraceSingleForObjects` :`Start` (`SceneComponent.GetSocketLocation` (`self.Mesh`) "head") :`End` (`self.K2_GetActorLocation` (`self.CurrentTarget`)) :`ObjectTypes` (`|MakeArray` "ObjectTypeQuery1" "ObjectTypeQuery2" :!type "EObjectTypeQuery Enum") :`DrawDebugType` "ForOneFrame"))
        (if _returnvalue_2
          (`KismetSystemLibrary.PrintString` (`KismetStringLibrary.Concat_StrStr` (`KismetSystemLibrary.GetDisplayName` (`.HitActor` (`GameplayStatics.BreakHitResult` _outhit))) "BlockedSubject"))
          (else
            (set `local.SeePlayer` true))))
      (:`then_1`
        (bind (_keypin _valuepin) (`|MapForEach` (`self.AllAvailableAction`))
          (:`then`
            (if (`.SightShouldNotBlocked_13_E49E34D746D0C90FEE71B89E885A711C` (break `/Game/System/GameCharacter/Enemies/Struct_ActionInformation` _valuepin))
              (if (`local.SeePlayer`)
                (if (and (> _returnvalue (`.MinRange_5_86E444EB48F2E18AFF073881EC479F75` (break `/Game/System/GameCharacter/Enemies/Struct_ActionInformation` _valuepin))) (<= _returnvalue (`.MaxRange_7_69E76BFC493182C5C2966FA351402495` (break `/Game/System/GameCharacter/Enemies/Struct_ActionInformation` _valuepin)))) :!label _label
                  (for _ (range (break `/Game/System/GameCharacter/Enemies/Struct_ActionInformation` _valuepin))
                    (`KismetArrayLibrary.Array_Add` (`local.SavedString`) _keypin))))
              (else
                (goto _label))))
          (:`CompletedPin`
            (`KismetArrayLibrary.Array_Shuffle` (`local.SavedString`))
            (bind _output_get (set `local.FinalResult` (`KismetArrayLibrary.Array_Random` (`local.SavedString`))))
            (`KismetSystemLibrary.PrintString` (`KismetStringLibrary.Concat_StrStr` "Randomed action" _output_get) true true (struct :`G` 0.082103 :`B` 0.729167 :`A` 1.0))
            (return _output_get)))))
    (else
      (set `local.FinalResult` _lockaction)
      (set `self.LockAction` "")
      (return (`local.FinalResult`)))))

(fn `RemoveStatus`
  (params (TargetStatus :type "/Game/System/Status/Bp_BaseStatusPackage Object Reference"))
  (`|ExecutionSequence`
    (:`then_0`
      (switch `/Game/System/Status/Enum_StatusTag` (`/Game/System/Status/Bp_BaseStatusPackage.StatusTagV2` TargetStatus)
        (:`NewEnumerator5`
          (if (== TargetStatus (`self.LastestCharm`))
            (set `self.LastestCharm` null)))))
    (:`then_1`
      (`parent.RemoveStatus` TargetStatus))))

(fn `UserConstructionScript`
  (`parent.UserConstructionScript`)
  (for _array_element (`self.DropingItem`)
    (`/Engine/EditorBlueprintResources/StandardMacros.IsValid` (`.FakePreviewMesh_14_2AFD427842974B48555EC0A88D37A177` (break `/Game/System/Item/Struct_EnemyItemDrop` _array_element))
      (:`Is Valid`
        (bind _returnvalue (`AddComponent|NODE_AddStaticMeshComponent-0`))
        (`StaticMeshComponent.SetStaticMesh` _returnvalue (`.FakePreviewMesh_14_2AFD427842974B48555EC0A88D37A177` (break `/Game/System/Item/Struct_EnemyItemDrop` _array_element)))
        (`SceneComponent.K2_AttachToComponent` _returnvalue (`self.Mesh`) (`.AttachedMeshLocation_12_FBD2975240044B8354CAFC9D5A0638DE` (break `/Game/System/Item/Struct_EnemyItemDrop` _array_element)) "SnapToTarget" "SnapToTarget" "KeepWorld" true)))))