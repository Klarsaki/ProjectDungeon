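; Enemy area manager that populates one area and wakes its AI when a player enters an activator box on the server.
; Activation also notifies any area listing this one as PreviousArea to run its spawning.
; Spawning fills placeholders by absolute, random or pair-tag rules, reusing "Recycle"-tagged enemies of matching class before spawning new ones.
; GroupAlert alerts area enemies once; box-overlap helpers collect enemies and placeholders.
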(event `OnPreviousAreaTrigger`
  (`self.CalculateSpawningRule`))

(event `self.ReceiveBeginPlay`
  (bind _previousarea (`self.PreviousArea`))
  (if (`self.Debug_DisableSpawn`)
    (`self.SetActorEnableCollision` false)
    (else
      (`|ExecutionSequence`
        (:`then_0`
          (for _array_element (`self.ActivatorBox`)
            (`/Engine/EditorBlueprintResources/ActorMacros.Switch Has Authority`
              (:`Authority`
                (`self.SetActorEnableCollision` _array_element true)
                (add `self.OnActorBeginOverlap` _array_element (delegate `CustomEvent`)))
              (:`Remote`
                (`self.SetActorEnableCollision` _array_element false)
                (`self.SetActorTickEnabled` _array_element false)))))
        (:`then_1`
          (`/Engine/EditorBlueprintResources/ActorMacros.Switch Has Authority`
            (:`Authority`
              (`/Engine/EditorBlueprintResources/StandardMacros.IsValid` _previousarea
                (:`Is Valid`
                  (add `self.Ed_StartAreaLogic` _previousarea (delegate `OnPreviousAreaTrigger`)))))))))))

(event `CustomEvent` :!signature `self.OnActorBeginOverlap`
  (params (OverlappedActor :type "Actor Object Reference") (OtherActor :type "Actor Object Reference"))
  (if (`self.ActorHasTag` OtherActor "Player")
    (`self.Ed_StartAreaLogic`)
    (`KismetSystemLibrary.PrintString` "Activate logic here")
    (`self.ServerActivate Enemies Logic In Area`)
    ; Deactivate as player colided
    (for _array_element (`self.ActivatorBox`)
      (`self.SetActorEnableCollision` _array_element false)
      (`self.SetActorTickEnabled` _array_element false))))

(event `ServerActivate Enemies Logic In Area`
  (for _array_element (`self.AreaEnemies`)
    (`/Game/System/GameCharacter/Enemies/Bp_BaseEnemy.StartupAi` _array_element self)))

(event `GroupAlert`
  (params (AlertPosition :type "Vector Structure") (Agroyer :type "/Game/System/GameCharacter/Bp_BasePlayableCharacter Object Reference"))
  (if (not (`self.AreaAlerted`))
    (for _array_element (`self.AreaEnemies`)
      (`/Game/System/GameCharacter/Enemies/Bp_BaseEnemy.OnAlert` _array_element AlertPosition Agroyer))
    (set `self.AreaAlerted` true)))

(event `Start InitialSpawn`
  (bind _outactors (`GameplayStatics.GetAllActorsOfClass` "/Game/System/GameCharacter/Enemies/Bp_BaseEnemy.Bp_BaseEnemy_C"))
  (for _array_element _outactors
    (if (`/Game/System/GameCharacter/Enemies/Bp_BaseEnemy.MarkRecycleable` _array_element)
      (`KismetArrayLibrary.Array_Add` (`self.UseableActors`) _array_element)))
  ; Comment
  (`self.CalculateSpawningRule`))

(fn `AutoCollectEnemiesInArea`
  (bind _areacapturereference (`self.AreaCaptureReference`))
  (bind _returnvalue (`SceneComponent.K2_GetComponentLocation` _areacapturereference))
  (bind _returnvalue_2 (* (`SceneComponent.K2_GetComponentScale` (`self.AreaCaptureReference`)) (`BoxComponent.BoxExtent` _areacapturereference)))
  (`KismetSystemLibrary.DrawDebugBox` _returnvalue _returnvalue_2 (struct :`R` 1.0 :`G` 1.0 :`B` 1.0 :`A` 1.0) (`SceneComponent.K2_GetComponentRotation` _areacapturereference) 1.0)
  (`|ExecutionSequence`
    (:`then_0`
      (bind _outactors (`KismetSystemLibrary.BoxOverlapActors` _returnvalue _returnvalue_2 (`|MakeArray` "ObjectTypeQuery3" :!type "EObjectTypeQuery Enum") "/Game/System/GameCharacter/Enemies/Bp_BaseEnemy.Bp_BaseEnemy_C"))
      (set `self.FoundedActor` _outactors)
      (`KismetSystemLibrary.PrintString` (`KismetStringLibrary.Conv_IntToString` (`KismetArrayLibrary.Array_Length` _outactors))))
    (:`then_1`
      (bind _outactors_2 (`KismetSystemLibrary.BoxOverlapActors` _returnvalue _returnvalue_2 (`|MakeArray` "ObjectTypeQuery8" :!type "EObjectTypeQuery Enum") "/Game/System/GameCharacter/Enemies/EnemyPlaceHolder.EnemyPlaceHolder_C"))
      (for _array_element _outactors_2
        (bind _asenemy_place_holder (cast `/Game/System/GameCharacter/Enemies/EnemyPlaceHolder` _array_element))
        (`KismetArrayLibrary.Array_AddUnique` (`self.TargetPlaceholder`) _asenemy_place_holder)
        ; AutoAddPairtag
        (switch `/Game/System/GameCharacter/Enemies/Enum_SpawningRate` (`/Game/System/GameCharacter/Enemies/EnemyPlaceHolder.SpawningRule` _asenemy_place_holder)
          (:`NewEnumerator1`
            (bind _pairtag (`/Game/System/GameCharacter/Enemies/EnemyPlaceHolder.PairTag` _asenemy_place_holder))
            (if (not (`.ReturnValue` (`BlueprintMapLibrary.Map_Find` (`self.SpawnForEachPairTag`) _pairtag)))
              (`BlueprintMapLibrary.Map_Add` (`self.SpawnForEachPairTag`) _pairtag))))))))

(fn `CalculateSpawningRule`
  (locals (RandomSpawn :type "Array of /Game/System/GameCharacter/Enemies/EnemyPlaceHolder Object Reference") (SpawnedUnique :type "Array of /Game/System/GameCharacter/Enemies/EnemyPlaceHolder Object Reference") (EachPairSpawner :type "Map of Name to /Game/System/GameCharacter/Enemies/Struct_PlaceHolderPair Structure") (IntCount :type Integer :default 0) (NewLocalVar :type "/Game/System/GameCharacter/Enemies/Bp_BaseEnemy Object Reference") (LocalPair :type "Array of /Game/System/GameCharacter/Enemies/EnemyPlaceHolder Object Reference"))
  (bind _eachpairspawner (`local.EachPairSpawner`))
  (`|ExecutionSequence`
    (:`then_0`
      (for _array_element (`self.TargetPlaceholder`)
        (switch `/Game/System/GameCharacter/Enemies/Enum_SpawningRate` (`/Game/System/GameCharacter/Enemies/EnemyPlaceHolder.SpawningRule` _array_element)
          (:`NewEnumerator0`
            (`KismetArrayLibrary.Array_Add` (`local.SpawnedUnique`) _array_element))
          (:`NewEnumerator1`
            (bind _pairtag (`/Game/System/GameCharacter/Enemies/EnemyPlaceHolder.PairTag` _array_element))
            (bind (_value _returnvalue) (`BlueprintMapLibrary.Map_Find` _eachpairspawner _pairtag))
            (if _returnvalue
              (`KismetArrayLibrary.Array_Add` (break `/Game/System/GameCharacter/Enemies/Struct_PlaceHolderPair` _value) _array_element)
              (else
                (`BlueprintMapLibrary.Map_Add` _eachpairspawner _pairtag (make `/Game/System/GameCharacter/Enemies/Struct_PlaceHolderPair` (`|MakeArray` _array_element))))))
          (:`NewEnumerator2`
            (`KismetArrayLibrary.Array_Add` (`local.RandomSpawn`) _array_element)))))
    (:`then_1`
      (bind _outactors (`GameplayStatics.GetAllActorsOfClassWithTag` "/Game/System/GameCharacter/Enemies/Bp_BaseEnemy.Bp_BaseEnemy_C" "Recycle"))
      (bind _output_get (set `self.UseableActors` _outactors))
      (`KismetSystemLibrary.PrintString` (`KismetStringLibrary.Conv_IntToString` (`KismetArrayLibrary.Array_Length` _output_get))))
    (:`then_2`
      ; Unique
      (set `local.IntCount` 0)
      (for _array_element_2 (`local.SpawnedUnique`)
        (`self.SpawnToTarget` _array_element_2 (`local.IntCount`))))
    (:`then_3`
      ; Random
      (`KismetArrayLibrary.Array_Shuffle` (`local.RandomSpawn`))
      (set `local.IntCount` 0)
      (for _index (range (`self.RandomSpawnWithinAmount`))
        (`self.SpawnToTarget` (`|GetArrayItem` (`local.RandomSpawn`) _index) (`local.IntCount`))))
    (:`then_4`
      ; Pair
      (bind (_keypin _valuepin) (`|MapForEach` (`local.EachPairSpawner`))
        (:`then`
          (set `local.IntCount` 0)
          (bind _output_get_2 (set `local.LocalPair` (break `/Game/System/GameCharacter/Enemies/Struct_PlaceHolderPair` _valuepin)))
          (`KismetArrayLibrary.Array_Shuffle` _output_get_2)
          (for _index_2 (range (`BlueprintMapLibrary.Map_Find` (`self.SpawnForEachPairTag`) _keypin))
            (`self.SpawnToTarget` (`|GetArrayItem` (`local.LocalPair`) _index_2) (`local.IntCount`))))))
    (:`then_5`
      (`KismetArrayLibrary.Array_Clear` (`self.UseableActors`)))))

(fn `ClearFounded`
  (`KismetArrayLibrary.Array_Clear` (`self.FoundedActor`)))

(fn `ConfirmPick`
  (for _array_element (`self.FoundedActor`)
    (`KismetArrayLibrary.Array_AddUnique` (`self.AreaEnemies`) (cast `/Game/System/GameCharacter/Enemies/Bp_BaseEnemy` _array_element :!pure true))))

(fn `SpawnToTarget`
  (params (InputPin :type "/Game/System/GameCharacter/Enemies/EnemyPlaceHolder Object Reference") (int :type "Integer (by ref)"))
  (locals (UsableActor :type "Array of /Game/System/GameCharacter/Enemies/Bp_BaseEnemy Object Reference") (IntCount :type Integer) (NewLocalVar :type "/Game/System/GameCharacter/Enemies/Bp_BaseEnemy Object Reference"))
  (bind _int (`local.Int`))
  (bind _targetspawntype (`/Game/System/GameCharacter/Enemies/EnemyPlaceHolder.TargetSpawnType` InputPin))
  (bind _newlocalvar (`local.NewLocalVar`))
  (bind _additionalitem (`/Game/System/GameCharacter/Enemies/EnemyPlaceHolder.AdditionalItem` InputPin))
  (bind _output (`|GetArrayItem` (`self.UseableActors`) (`local.Int`)))
  (`|VariableSetRef` (`local.int`))
  (`KismetSystemLibrary.PrintString` "Hello" :!label _label)
  (`/Engine/EditorBlueprintResources/StandardMacros.IsValid` InputPin
    (:`Is Valid`
      (`/Engine/EditorBlueprintResources/StandardMacros.IsValid` _output
        (:`Is Valid`
          (if (`KismetSystemLibrary.IsValidClass` _targetspawntype)
            (bind _output_get (set `local.NewLocalVar` _output))
            (if (`GameplayStatics.ObjectIsA` _output_get _targetspawntype)
              (`KismetArrayLibrary.Array_Remove` (`self.UseableActors`) _int)
              (`/Game/System/GameCharacter/Enemies/Bp_BaseEnemy.StartRecycleUnit` _newlocalvar (`local.InputPin`) _additionalitem)
              (`KismetArrayLibrary.Array_AddUnique` (`self.AreaEnemies`) _newlocalvar)
              (else
                (`/Engine/EditorBlueprintResources/StandardMacros.IncrementInt` _int
                  (:`  `
                    (goto _label)))))))
        (:`Is Not Valid`
          (bind _returnvalue (`|SpawnActorFromClass` _targetspawntype (`self.GetTransform` (`local.InputPin`)) "Undefined" "MultiplyWithRoot" null null))
          (`/Game/System/GameCharacter/Enemies/Bp_BaseEnemy.StartRecycleUnit` _returnvalue (`local.InputPin`) _additionalitem))))))

(fn `UserConstructionScript`)