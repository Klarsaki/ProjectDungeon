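; Interactable owned by a playable character that lets another character revive it through a timed interaction.
; AsInteracted blocks further interaction, binds to the reviver's death, damage and interact-release events, and passes a revive timer handle to the reviver.
; Timer completion calls CharacterRevived on the owner and disables collision.
; Interruptions unbind events, reopen interaction and toggle collision off for one tick, while AllowRules rejects the owner as interactor.
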(event `self.ReceiveBeginPlay`
  (`parent.ReceiveBeginPlay`)
  (`self.SetActorEnableCollision` false))

(event `self.AsInteracted`
  (params (Interacter :type "/Game/System/GameCharacter/AC_InteractedQueueReader Object Reference"))
  (set `self.ServerAllowsInteract` false)
  (`self.RemoveFromAllRemainingClient` (`self.interactedList`))
  (bind _asbp_base_playable_character (cast `/Game/System/GameCharacter/Bp_BasePlayableCharacter` (`ActorComponent.GetOwner` Interacter)))
  (set `self.As Bp Base Playable Character` _asbp_base_playable_character)
  (`KismetSystemLibrary.PrintString` "Hello")
  (`self.AllStopCondition`))

(event `AllStopCondition`
  (bind _as_bp_base_playable_character (`self.As Bp Base Playable Character`))
  (add `/Game/System/GameCharacter/Bp_BaseCharacter.Ed_DeathCall` _as_bp_base_playable_character (delegate `Ed_DeathCall_Event`))
  (add `/Game/System/GameCharacter/Bp_BaseCharacter.Ed_PostRecievDamage` _as_bp_base_playable_character (delegate `Ed_PostRecievDamage_Event`))
  (add `/Game/System/GameCharacter/Bp_BasePlayableCharacter.Ed_InteractRelease` _as_bp_base_playable_character (delegate `Ed_InteractRelease_Event`))
  (bind _returnvalue (`KismetSystemLibrary.K2_SetTimerDelegate` (delegate `OnReviveSuccess`) 7.0))
  (bind _output_get (set `self.NewVar_0` _returnvalue))
  (`/Game/System/GameCharacter/Bp_BasePlayableCharacter.PlayerRevivingSomeOne` (`self.As Bp Base Playable Character`) true (cast `/Game/System/GameCharacter/Bp_BasePlayableCharacter` (`self.GetOwner`) :!pure true) _output_get))

(event `Ed_DeathCall_Event`
  (`self.StopInteraction`))

(event `Ed_PostRecievDamage_Event`
  (params (ResultDamage :type "Float (double-precision)") (SourceOfDmg :type "Actor Object Reference"))
  (if (> ResultDamage 0.0)
    (`self.StopInteraction`)))

(event `OnReviveSuccess`
  (`/Game/System/GameCharacter/Bp_BasePlayableCharacter.PlayerRevivingSomeOne` :`self` (`self.As Bp Base Playable Character`))
  (bind _asbp_base_playable_character (cast `/Game/System/GameCharacter/Bp_BasePlayableCharacter` (`self.GetOwner`)))
  (`/Game/System/GameCharacter/Bp_BasePlayableCharacter.CharacterRevived` _asbp_base_playable_character)
  (`self.SetActorEnableCollision` false)
  (`self.NormalStop`))

(event `Ed_InteractRelease_Event`
  (`self.StopInteraction`))

(event `NormalStop`
  (bind _as_bp_base_playable_character (`self.As Bp Base Playable Character`))
  (remove `/Game/System/GameCharacter/Bp_BaseCharacter.Ed_DeathCall` _as_bp_base_playable_character (delegate `Ed_DeathCall_Event`) :!label _label)
  (remove `/Game/System/GameCharacter/Bp_BaseCharacter.Ed_PostRecievDamage` _as_bp_base_playable_character (delegate `Ed_PostRecievDamage_Event`))
  (remove `/Game/System/GameCharacter/Bp_BasePlayableCharacter.Ed_InteractRelease` _as_bp_base_playable_character (delegate `Ed_InteractRelease_Event`))
  (`KismetSystemLibrary.PrintString` "Cancled")
  (set `self.ServerAllowsInteract` true))

(event `StopInteraction`
  (`|ExecutionSequence`
    (:`then_0`
      (goto _label))
    (:`then_1`
      (`self.SetActorEnableCollision` false)
      (`/Game/System/GameCharacter/Bp_BasePlayableCharacter.PlayerRevivingSomeOne` :`self` (`self.As Bp Base Playable Character`))
      (`KismetSystemLibrary.DelayUntilNextTick`)
      (`self.SetActorEnableCollision` true))))

(fn `AllowRules`
  (params (Interactor :type "Actor Object Reference"))
  (returns (NewParam :type Boolean))
  (bind _newparam (`parent.AllowRules` Interactor))
  (return (and _newparam (!= Interactor (`self.GetOwner`)))))

(fn `UserConstructionScript`
  (`parent.UserConstructionScript`))