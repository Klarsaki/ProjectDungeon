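; Interactable world object that offers itself to playable characters entering its sphere and withdraws once interacted with.
; Server-side overlaps maintain InteractedList and call client-named events that update the ACInteractedQueueReader of locally viewed characters.
; AsInteracted blocks further interaction, disables sphere overlaps through MulticastDisable and removes itself from remaining characters' queues.
; StartEnable and EnablingInteractObject only toggle actor tick, not the overlap logic.
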(event `self.ReceiveBeginPlay`
  (if (not (`self.StartEnable`))
    (`self.SetActorTickEnabled` false)))

(event `EnablingInteractObject`
  (`self.SetActorTickEnabled` true))

(event `self.Sphere.OnComponentBeginOverlap`
  (params (OverlappedComponent :type "PrimitiveComponent Object Reference") (OtherActor :type "Actor Object Reference") (OtherComp :type "PrimitiveComponent Object Reference") (OtherBodyIndex :type Integer) (bFromSweep :type Boolean) (SweepResult :type "HitResult Structure (by ref)"))
  (`/Engine/EditorBlueprintResources/ActorMacros.Switch Has Authority`
    (:`Authority`
      (if (`self.ServerAllowsInteract`)
        (`KismetArrayLibrary.Array_AddUnique` (`self.interactedList`) OtherActor)
        (`self.Add interactionToClient` OtherActor)))))

(event `Add interactionToClient`
  (params (Object :type "Actor Object Reference"))
  (bind _asbp_base_playable_character (cast `/Game/System/GameCharacter/Bp_BasePlayableCharacter` Object))
  (`/Engine/EditorBlueprintResources/StandardMacros.IsValid` (`Pawn.GetLocalViewingPlayerController` _asbp_base_playable_character)
    (:`Is Valid`
      (`/Game/System/GameCharacter/AC_InteractedQueueReader.AddIncomingInteractable` (`/Game/System/GameCharacter/Bp_BasePlayableCharacter.AC_InteractedQueueReader` _asbp_base_playable_character) self))))

(event `self.Sphere.OnComponentEndOverlap`
  (params (OverlappedComponent :type "PrimitiveComponent Object Reference") (OtherActor :type "Actor Object Reference") (OtherComp :type "PrimitiveComponent Object Reference") (OtherBodyIndex :type Integer))
  (`/Engine/EditorBlueprintResources/ActorMacros.Switch Has Authority`
    (:`Authority`
      (if (`self.ServerAllowsInteract`)
        (`KismetArrayLibrary.Array_RemoveItem` (`self.interactedList`) OtherActor)
        (`self.RemoveatClient` OtherActor)))))

(event `AsInteracted`
  (params (Interacter :type "/Game/System/GameCharacter/AC_InteractedQueueReader Object Reference"))
  (set `self.ServerAllowsInteract` false)
  (`self.MulticastDisable` Interacter)
  (`self.RemoveFromAllRemainingClient` (`self.interactedList`)))

(event `RemoveAtClient`
  (params (Object :type "Actor Object Reference"))
  (bind _asbp_base_playable_character (cast `/Game/System/GameCharacter/Bp_BasePlayableCharacter` Object))
  (`/Engine/EditorBlueprintResources/StandardMacros.IsValid` (`Pawn.GetLocalViewingPlayerController` _asbp_base_playable_character)
    (:`Is Valid`
      (`/Game/System/GameCharacter/AC_InteractedQueueReader.RemoveInteractable` (`/Game/System/GameCharacter/Bp_BasePlayableCharacter.AC_InteractedQueueReader` _asbp_base_playable_character) self))))

(event `RemoveFromAllRemainingClient`
  (params (interactedList :type "Array of Actor Object Reference"))
  (for _array_element interactedList
    (`self.RemoveatClient` _array_element))
  (`/Engine/EditorBlueprintResources/ActorMacros.Switch Has Authority`
    (:`Authority`
      (`KismetArrayLibrary.Array_Clear` (`self.interactedList`)))))

(event `MulticastDisable`
  (params (InputPin :type "/Game/System/GameCharacter/AC_InteractedQueueReader Object Reference"))
  (set `PrimitiveComponent.bGenerateOverlapEvents` false (`self.Sphere`)))

(fn `NewFunction`)

(fn `UserConstructionScript`)