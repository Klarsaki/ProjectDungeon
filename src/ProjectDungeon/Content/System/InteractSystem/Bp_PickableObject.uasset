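; Pickable world object that grants an item to a playable character's inventory when interacted with.
; It extends the parent's AsInteracted event, then casts the interacter's owner to Bp_BasePlayableCharacter.
; If GrantedObject is valid, it adds that item in the configured Amount through the character's BpInventoryHolder.
; The graph does not remove or disable the object after granting.
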(event `self.AsInteracted`
  (params (Interacter :type "/Game/System/GameCharacter/AC_InteractedQueueReader Object Reference"))
  (`parent.AsInteracted` Interacter)
  (`self.AddItemToTarget` Interacter))

(event `AddItemToTarget`
  (params (Interacter :type "/Game/System/GameCharacter/AC_InteractedQueueReader Object Reference"))
  (bind _grantedobject (`self.GrantedObject`))
  (bind _asbp_base_playable_character (cast `/Game/System/GameCharacter/Bp_BasePlayableCharacter` (`ActorComponent.GetOwner` Interacter)))
  (`/Engine/EditorBlueprintResources/StandardMacros.IsValid` _grantedobject
    (:`Is Valid`
      (`/Game/System/Ingame/Inventory/Bp_InventoryHolder.AddItemToInventory` (`/Game/System/GameCharacter/Bp_BasePlayableCharacter.Bp_InventoryHolder` _asbp_base_playable_character) _grantedobject (`self.Amount`)))))

(fn `UserConstructionScript`
  (`parent.UserConstructionScript`))