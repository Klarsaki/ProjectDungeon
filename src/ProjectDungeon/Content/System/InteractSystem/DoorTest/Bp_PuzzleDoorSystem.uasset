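; Puzzle door actor that moves a TargetCell actor vertically according to how many notices are active.
; ActivateNotice and UnactivateNotice adjust NoticeCount and start an update toward a height that steps up from the cached BeginPlay position per count.
; Unless Locked, Tick shifts the cell with local Z offsets, rising slower than it falls, and stops updating once it crosses the target height.
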(event `self.ReceiveBeginPlay`
  (set `self.CacheLo` (`self.K2_GetActorLocation` (`self.TargetCell`))))

(event `self.ReceiveTick`
  (params (DeltaSeconds :type "Float (single-precision)"))
  (bind _targetcell (`self.TargetCell`))
  (bind (_returnvalue_x _returnvalue_y _returnvalue_z) (`KismetMathLibrary.BreakVector` (`self.K2_GetActorLocation` (`self.TargetCell`))))
  (bind (_returnvalue_x_2 _returnvalue_y_2 _returnvalue_z_2) (`KismetMathLibrary.BreakVector` (`self.K2_GetActorLocation` (`self.TargetCell`))))
  (bind (_returnvalue_x_3 _returnvalue_y_3 _returnvalue_z_3) (`KismetMathLibrary.BreakVector` (`self.K2_GetActorLocation` (`self.TargetCell`))))
  (bind _z (.z (+ (`self.CacheLo`) (`KismetMathLibrary.MakeVector` 0.0 0.0 (* 80 (`self.NoticeCount`))))))
  (if (`self.Locked`)
    _
    (elif (`self.UpdateOn`)
      (if (>= _returnvalue_z_2 _z)
        (`self.K2_AddActorLocalOffset` _targetcell (`KismetMathLibrary.MakeVector` 0.0 0.0 (* -120.0 DeltaSeconds)) false false)
        (if (not (>= _returnvalue_z _z))
          (set `self.UpdateOn` false))
        (else
          (`self.K2_AddActorLocalOffset` _targetcell (`KismetMathLibrary.MakeVector` 0.0 0.0 (* DeltaSeconds 50.0)) false false)
          (if (>= _returnvalue_z_3 _z)
            (set `self.UpdateOn` false)))))))

(event `ActivateNotice`
  (`/Engine/EditorBlueprintResources/StandardMacros.IncrementInt` (`self.NoticeCount`)
    (:`  `
      (`self.UpdateCell`))))

(event `UpdateCell`
  (set `self.UpdateOn` true))

(event `UnactivateNotice`
  (`/Engine/EditorBlueprintResources/StandardMacros.DecrementInt` (`self.NoticeCount`)
    (:`  `
      (`self.UpdateCell`))))

(fn `UserConstructionScript`)