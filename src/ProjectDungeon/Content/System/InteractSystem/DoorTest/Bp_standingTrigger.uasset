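; Bp_standingTrigger is a standing trigger that reports to a PuzzleMaster while a playable character is inside its sphere.
; The first Bp_BasePlayableCharacter to enter sets the Activated flag and calls ActivateNotice on the PuzzleMaster.
; When an overlap ends, it checks for remaining playable characters and only clears the flag and calls UnactivateNotice once none are left.
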(event `self.Sphere.OnComponentBeginOverlap`
  (params (OverlappedComponent :type "PrimitiveComponent Object Reference") (OtherActor :type "Actor Object Reference") (OtherComp :type "PrimitiveComponent Object Reference") (OtherBodyIndex :type Integer) (bFromSweep :type Boolean) (SweepResult :type "HitResult Structure (by ref)"))
  (if (and (`GameplayStatics.ObjectIsA` OtherActor "/Game/System/GameCharacter/Bp_BasePlayableCharacter.Bp_BasePlayableCharacter_C") (not (`self.Activated`)))
    (set `self.Activated` true)
    (`/Game/System/InteractSystem/DoorTest/Bp_PuzzleDoorSystem.ActivateNotice` (`self.PuzzleMaster`))))

(event `self.Sphere.OnComponentEndOverlap`
  (params (OverlappedComponent :type "PrimitiveComponent Object Reference") (OtherActor :type "Actor Object Reference") (OtherComp :type "PrimitiveComponent Object Reference") (OtherBodyIndex :type Integer))
  (if (`self.Activated`)
    (`/Engine/EditorBlueprintResources/StandardMacros.IsValid` (`|GetArrayItem` (`PrimitiveComponent.GetOverlappingActors` (`self.Sphere`) "/Game/System/GameCharacter/Bp_BasePlayableCharacter.Bp_BasePlayableCharacter_C"))
      (:`Is Not Valid`
        (set `self.Activated` false)
        (`/Game/System/InteractSystem/DoorTest/Bp_PuzzleDoorSystem.UnactivateNotice` (`self.PuzzleMaster`))))))

(fn `UserConstructionScript`)