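; Preview character actor that shows a selectable class model (Tank, Attacker, Rogue or Mage) with a name label.
; RefreshCharIndex maps the one-based CurrentCharIndex to a skeletal mesh and looping idle animation, running on BeginPlay and whenever NewPreviewChar changes the index.
; SetName stores the name, then tells every preview character in the level to write its own MyName to its TextRender.
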(event `SetName`
  (params (`My Name` :type Name))
  (set `self.My Name` `My Name`)
  (bind _outactors (`GameplayStatics.GetAllActorsOfClass` "Bp_PreviewCharacter_C"))
  (for _array_element _outactors
    (`self.DisplayName` _array_element)))

(event `DisplayName`
  (`TextRenderComponent.K2_SetText` (`self.TextRender`) (`KismetTextLibrary.Conv_NameToText` (`self.My Name`))))

(event `self.ReceiveBeginPlay`
  (`KismetSystemLibrary.PrintString` "PlayWhenJoin")
  (`self.RefreshCharIndex`))

(event `NewPreviewChar`
  (params (NewParam :type Integer))
  (set `self.CurrentCharIndex` NewParam)
  (`self.RefreshCharIndex`))

(event `RefreshCharIndex`
  (bind _returnvalue (- (`self.CurrentCharIndex`) 1))
  (`SkeletalMeshComponent.SetSkeletalMeshAsset` (`self.Mesh`) (select `int` _returnvalue :`0` "/Game/Characters/PlayerChar/Tank/SKM_Tank.SKM_Tank" :`1` "/Game/Characters/PlayerChar/AttackerV2/SKM_Attacker.SKM_Attacker" :`2` "/Game/Characters/PlayerChar/Rogue/SKM_Rogue.SKM_Rogue" :`3` "/Game/Characters/PlayerChar/Mage2/SKM_Mage.SKM_Mage" :!type "SkeletalMesh Object Reference"))
  (`SkeletalMeshComponent.PlayAnimation` (`self.Mesh`) (select `int` _returnvalue :`0` "/Game/Characters/PlayerChar/Tank/Anim_Idle.Anim_Idle" :`1` "/Game/Characters/PlayerChar/AttackerV2/Anim_Idle01_Anim.Anim_Idle01_Anim" :`2` "/Game/Characters/PlayerChar/Rogue/Anim_Idle_Knife.Anim_Idle_Knife" :`3` "/Game/Characters/PlayerChar/Mage2/Anim_Idle.Anim_Idle" :!type "AnimationAsset Object Reference") true))

(fn `UserConstructionScript`)