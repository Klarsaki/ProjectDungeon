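; Player controller for the lobby, handling player setup and character selection.
; BeginPlay copies the player name from the game instance to the preview pawn and shows the preparation widget for local controllers.
; Possess notifies the lobby game mode and, after a short delay, switches view to the MainCam-tagged camera and adds a debug tracker widget.
; Selection changes go through ServerSetPreviewChar, which updates the PlayerState and preview character.
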(event `self.ReceiveBeginPlay`
  (bind _asbp_preview_character (cast `/Game/System/Bp_PreviewCharacter` (`self.K2_GetPawn`) :!pure true))
  (bind _asbp_dun_game_instance (cast `/Game/System/Bp_DunGameInstance` (`GameplayStatics.GetGameInstance`)))
  (bind _output_get (set `self.MyName` (`/Game/System/Bp_DunGameInstance.PlayerName` _asbp_dun_game_instance)))
  (`/Engine/EditorBlueprintResources/StandardMacros.IsValid` _asbp_preview_character
    (:`Is Valid`
      (`/Game/System/Bp_PreviewCharacter.SetName` _asbp_preview_character _output_get))
    (:`Is Not Valid`
      _))
  (`|ExecutionSequence`
    (:`then_0`
      (if (`self.IsLocalController`)
        (bind _returnvalue (`|CreateWidget` "/Game/System/Widget/WG_InLobbyPreparation.WG_InLobbyPreparation_C" self))
        (`UserWidget.AddToViewport` _returnvalue 0)))))

(event `self.ReceivePossess`
  (params (PossessedPawn :type "Pawn Object Reference"))
  (`self.ConnectToCam`)
  (`/Game/System/Inlobby/GM_LobbyGamemode.OnJoin` (cast `/Game/System/Inlobby/GM_LobbyGamemode` (`GameplayStatics.GetGameMode`) :!pure true)))

(event `ConnectToCam`
  (`KismetSystemLibrary.Delay` 1.0)
  (bind _outactors (`GameplayStatics.GetAllActorsWithTag` "MainCam"))
  (bind _ascamera_actor (cast `CameraActor` (`|GetArrayItem` _outactors) :!pure true))
  (`self.SetViewTargetWithBlend` (`PlayerCameraManager.GetOwningPlayerController` (`self.PlayerCameraManager`)) _ascamera_actor 0.0 "VTBlend_Linear" 0.0 false)
  (`ActorComponent.SetActive` (`CameraActor.CameraComponent` _ascamera_actor) true false)
  (bind _returnvalue (`|CreateWidget` "/Game/System/Widget/Debug_TrackerWIdget.Debug_TrackerWIdget_C" self))
  (`UserWidget.AddToViewport` _returnvalue 0))

(event `self.ReceiveTick`
  (params (DeltaSeconds :type "Float (single-precision)")))

(event `SetSelectedCharacter`
  (params (NewCharIndex :type Integer))
  (if (!= NewCharIndex (`/Game/System/PS_DungeonPlayerState.SelectedChar` (cast `/Game/System/PS_DungeonPlayerState` (`self.PlayerState`) :!pure true)))
    (`self.ServerSetPreviewChar` NewCharIndex)))

(event `ServerSetPreviewChar`
  (params (NewParam :type Integer))
  (bind _output_get (set `/Game/System/PS_DungeonPlayerState.SelectedChar` NewParam (cast `/Game/System/PS_DungeonPlayerState` (`self.PlayerState`) :!pure true)))
  (`KismetSystemLibrary.PrintString` (`KismetStringLibrary.Conv_IntToString` _output_get))
  (`/Game/System/Bp_PreviewCharacter.NewPreviewChar` (cast `/Game/System/Bp_PreviewCharacter` (`self.K2_GetPawn`) :!pure true) NewParam))

(fn `UserConstructionScript`)