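; Lobby game mode that tracks joining players and launches the match.
; PostLogin stores the network player count in JoinedPlayer and calls the EDLoggedIn dispatcher.
; GameStart server-travels to LV_GameLevel001, while OnLogout only prints a debug string.
; ChoosePlayerStart override picks the first PlayerStart with no pawn in a tiny overlap sphere, falling back to the first one found.
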(event `self.K2_PostLogin`
  (params (NewPlayer :type "PlayerController Object Reference"))
  (set `self.JoinedPlayer` (`AdvancedSessionsLibrary.GetNumberOfNetworkPlayers`))
  (`self.ED_LoggedIn`))

(event `OnJoin`)

(event `GameStart`
  (`AdvancedSessionsLibrary.ServerTravel` "LV_GameLevel001"))

(event `self.K2_OnLogout`
  (params (ExitingController :type "Controller Object Reference"))
  (`KismetSystemLibrary.PrintString` "LogoutCalled"))

(fn `ChoosePlayerStart`
  (params (Player :type "Controller Object Reference"))
  (returns (ReturnValue :type "Actor Object Reference"))
  (bind _outactors (`GameplayStatics.GetAllActorsOfClass` "/Script/Engine.PlayerStart"))
  (for _array_element _outactors
    (bind (_outactors_2 _returnvalue) (`KismetSystemLibrary.SphereOverlapActors` (`self.K2_GetActorLocation` _array_element) 1.0 (`|MakeArray` "ObjectTypeQuery3" :!type "EObjectTypeQuery Enum") null _outactors))
    (if (not _returnvalue)
      (return _array_element)))
  (return (`|GetArrayItem` _outactors)))

(fn `UserConstructionScript`)