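; Base weapon Blueprint that attaches to its owning character's hand sockets and handles equip, unequip and melee hit damage, with input and hit events left empty as hooks.
; Equipping briefly sets the holder's action state, unhides the weapon and plays a montage.
; An authority-only timed hitbox toggles capsule overlaps, caching targets to prevent repeat hits.
; Hits use the holder's damage calculator, halve player-versus-player damage, apply knock force and stun non-players.
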(event `self.ReceiveBeginPlay`
  ;[0.15 0.15 0.15 0.5 146] AttachWhenWeapon'sBeginPlay
  (`KismetSystemLibrary.Delay` 0.2)
  (`self.WeaponSetup` (cast `/Game/System/GameCharacter/Bp_BaseCharacter` (`self.GetOwner`) :!pure true))
  (`KismetSystemLibrary.PrintString` "SetwpOwner"))

(event `WeaponSetup`
  (params (Holder :type "/Game/System/GameCharacter/Bp_BaseCharacter Object Reference"))
  ;[0.15 0.15 0.15 0.5 146] AttachWhenWeapon'sBeginPlay
  (bind _output_get (set `self.Holder` Holder))
  (`self.K2_AttachToActor` _output_get "None" "SnapToTarget" "SnapToTarget" "KeepRelative")
  (`SceneComponent.K2_AttachToComponent` (`self.RHand`) (`Character.Mesh` (`self.Holder`)) (`self.AttatchRBoneName`) "SnapToTarget" "SnapToTarget" "KeepWorld" true)
  (`SceneComponent.K2_AttachToComponent` (`self.LHand`) (`Character.Mesh` (`self.Holder`)) (`self.AttatchLBoneName`) "SnapToTarget" "SnapToTarget" "KeepWorld" true)
  (`KismetSystemLibrary.PrintString` "AttachToOwner"))

(event `StopActiving`
  (`self.SetActorHiddenInGame` true) ; This shit run on server
  (`self.Ed_StopWeaponActiving`))

(event `ServerStartEquipActive`
  (`self.SetActorHiddenInGame` false) ; This shit run on server
  (`self.PlayActiveAnimation`))

(event `StartActiveEquip`
  (bind _asbp_base_playable_character (cast `/Game/System/GameCharacter/Bp_BasePlayableCharacter` (`self.Holder`)))
  (`/Game/System/GameCharacter/Bp_BasePlayableCharacter.SetActionStateByTimer` _asbp_base_playable_character 0.3 "ChangeWeapon" "NewEnumerator1" 1.0 true)
  (`KismetSystemLibrary.PrintString` "ActiveNewWeaponIndex" true true (struct :`R` 1.0 :`G` 0.674626 :`A` 1.0))
  (`self.ServerStartEquipActive`))

(event `PlayActiveAnimation`
  (`|PlayMontage` (`Character.Mesh` (`self.Holder`)) (`self.EquipInMontage`)))

(event `PrimaryInputTrigger`
  (params (isIn :type Boolean)))

(event `MiddleInputTrigger`
  (params (isIn :type Boolean)))

(event `SecondaryInputTrigger`
  (params (isIn :type Boolean)))

(event `SecondaryHolding`)

(event `ActivateHitboxWithTimer`
  (params (Duration :type "Float (double-precision)") (Index :type Integer))
  (`/Engine/EditorBlueprintResources/ActorMacros.Switch Has Authority`
    (:`Authority`
      (`self.SetEnableDamageBox` 0) ; ClearAnyEnable if thereis
      (if (> Duration 0.0)
        (`self.SetEnableDamageBox` Index true)
        (`KismetSystemLibrary.RetriggerableDelay` Duration)
        (`self.SetEnableDamageBox` Index)))))

(event `SetEnableDamageBox`
  (params (Variation :type Integer) (SetEnable :type Boolean))
  (`/Engine/EditorBlueprintResources/ActorMacros.Switch Has Authority`
    (:`Authority`
      (`self.AsEnableDamage` Variation SetEnable))))

(event `AsEnableDamage`
  (params (Variation :type Integer) (Set :type Boolean))
  ; Implement damage colision
  (if Set
    (switch `int` Variation
      (:`Default`
        (`KismetArrayLibrary.Array_Clear` (`self.AppliedCacheTarget`))
        (set `PrimitiveComponent.bGenerateOverlapEvents` true (`self.Capsule`))))
    (else
      (set `PrimitiveComponent.bGenerateOverlapEvents` false (`self.Capsule`)) ; DisableAllColisionHere
    )))

(event `self.Capsule.OnComponentBeginOverlap`
  (params (OverlappedComponent :type "PrimitiveComponent Object Reference") (OtherActor :type "Actor Object Reference") (OtherComp :type "PrimitiveComponent Object Reference") (OtherBodyIndex :type Integer) (bFromSweep :type Boolean) (SweepResult :type "HitResult Structure (by ref)"))
  ; DefaulHItboxOverlap
  (`/Engine/EditorBlueprintResources/ActorMacros.Switch Has Authority`
    (:`Authority`
      (bind _asbp_base_character (cast `/Game/System/GameCharacter/Bp_BaseCharacter` OtherActor))
      (bind (_returnvalue _returnvalue2 _isplayer) (`self.NewMacro` _asbp_base_character OtherActor _asbp_base_character))
      (if _returnvalue2
        (`KismetArrayLibrary.Array_AddUnique` (`self.AppliedCacheTarget`) _asbp_base_character)
        (bind _outputdamage (`/Game/System/GameCharacter/Bp_BaseCharacter.DamageCalculator` (`self.Holder`) _returnvalue _asbp_base_character null)) ; Damage calculator of actor
        (`KismetSystemLibrary.PrintString` (`KismetStringLibrary.Conv_DoubleToString` _outputdamage) true true (struct :`R` 1.0 :`B` 0.014564 :`A` 1.0))
        (`/Game/System/GameCharacter/Bp_BaseCharacter.Server_RequestApplyDamage` _asbp_base_character _outputdamage false self (0.0 0.0 0.0) (`self.PushForce`))
        (`self.OnDamageApplied` _asbp_base_character)
        (if _isplayer
          _
          (elif (> (`self.BaseStunDuration`) 0.0)
            (bind _returnvalue_2 (`|GenericCreateObject` "/Game/System/Status/Bp_BaseStatusPackage.Bp_BaseStatusPackage_C"))
            (`/Game/System/Status/Bp_BaseStatusPackage.SetupPackage` _returnvalue_2 "SimpleWeaponStun" "" 1 (`self.BaseStunDuration`) "NewEnumerator0" self (`self.Holder`) 0.0 0 false false)
            (message `/Game/System/GameCharacter/Int_StatusPackage.InterfaceApplyStatus` _asbp_base_character _returnvalue_2)))))))

(event `OnDamageApplied`
  (params (char :type "/Game/System/GameCharacter/Bp_BaseCharacter Object Reference"))
  ; DefaulHItboxOverlap
)

(fn `UserConstructionScript`)