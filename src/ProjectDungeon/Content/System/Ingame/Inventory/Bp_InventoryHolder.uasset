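; Inventory component for a playable character that tracks item counts in a map seeded from default items, which can be topped back up.
; Add and consume functions update counts and fire add, update or remove notifications, optionally keeping empty slots; consumption always removes one.
; UseItem validates stock, then routes the item's script class through server and all-client events, which construct and cache one UObject per class to run the effect.
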(event Custom|AtServer
  (params (NewParam :type Object%20Class%20Reference))
  (CallFunction|SpawntoAll NewParam))

(event Custom|SpawnToAll
  (params (NewParam :type Object%20Class%20Reference))
  (bind _returnvalue (Components|GetOwner))
  (bind _asbp_base_playable_character (Utilities|Casting|CastToBp_BasePlayableCharacter _returnvalue))
  (bind (_found _cachedone) (CallFunction|IsFunctionScriptCached NewParam))
  (if _found
    (Class|INTImplementingUsingItem|OnUsedItem(Message) _cachedone _asbp_base_playable_character)
    (Development|PrintString "CachedUsage")
    (else
      (bind _returnvalue_2 (Game|ConstructObjectfromClass NewParam))
      (Utilities|Array|Add (Variables|Default|GetCacheUsingScript) _returnvalue_2)
      (Class|INTImplementingUsingItem|OnUsedItem(Message) _returnvalue_2 _asbp_base_playable_character))))

(event Custom|DefaultItemReset
  (bind _dict_itemcontainer (Variables|Default|GetDict_ItemContainer))
  (for (_array_element _array_index) (Variables|Default|GetDefaultItem)
    (if (not (> (.Value (Utilities|Map|GetKeyValueByIndex _dict_itemcontainer _array_index)) (.maximumslot _array_element)))
      ;[0.15 0.15 0.15 0.5] Reset value if value is less than maximum
      (Utilities|Map|Add _dict_itemcontainer (.Key (Utilities|Map|GetKeyValueByIndex _dict_itemcontainer _array_index)) (.maximumslot _array_element)))))

(event Custom|ConstructionItemScript
  (params (InputPin :type Object%20Class%20Reference))
  (CallFunction|AtServer InputPin))

(event Custom|MultiFromServer_ConsumeItem
  (params (TargetToConsume :type PMA%20Item%20Data%20Object%20Reference) (IfNoTargetUseIndex :type Integer) (AmountToConsume :type Integer))
  (CallFunction|ConsumeItem TargetToConsume IfNoTargetUseIndex AmountToConsume))

(event EventBeginPlay
  (for _array_element (Variables|Default|GetDefaultItem)
    (Utilities|Map|Add (Variables|Default|GetDict_ItemContainer) (.item _array_element) (.maximumslot _array_element))))

(event EventTick
  (params (DeltaSeconds :type Float%20%28single-precision%29)))

(event Input|KeyboardEvents|DebugKeyC
  (params (Key :type Key%20Structure) (ActionValue :type Input%20Action%20Value%20Structure))
  (:Pressed
    (CallFunction|UseItem (Variables|Default|GetTest_DaPotion))))

(fn AddItemtoInventory
  (params (NewlyItem :type PMA%20Item%20Data%20Object%20Reference) (Amount :type Integer))
  (bind _dict_itemcontainer (Variables|Default|GetDict_ItemContainer))
  (bind (_value _returnvalue) (Utilities|Map|Find _dict_itemcontainer NewlyItem))
  (bind _returnvalue_2 (+ _value Amount))
  (Development|PrintString (Utilities|GetDisplayName NewlyItem))
  (Utilities|FlowControl|Sequence
    (:then_0
      (if (> Amount 0)
        (if _returnvalue
          (Utilities|Map|Add _dict_itemcontainer NewlyItem _returnvalue_2)
          (Default|CallEdItemUpdate NewlyItem _returnvalue_2)
          (else
            (Utilities|Map|Add _dict_itemcontainer NewlyItem Amount)
            (Default|CallEdItemAdded NewlyItem Amount)))))))

(fn RemoveItemfromInventory)

(fn ConsumeItem
  (params (TargetToConsume :type PMA%20Item%20Data%20Object%20Reference) (IfNoTargetUseIndex :type Integer) (AmountToConsume :type Integer))
  (bind _dict_itemcontainer (Variables|Default|GetDict_ItemContainer))
  (bind (_value _returnvalue) (Utilities|Map|Find _dict_itemcontainer TargetToConsume))
  (bind _returnvalue_2 (- _value 1))
  (Utilities|FlowControl|Sequence
    (:then_0
      (Utilities|IsValid TargetToConsume
        (:Is%20Valid
          (if _returnvalue
            (if (> _value 0)
              (if (Variables|/Game/System/Item/PMA_ItemData.PMA_ItemData_C|GetRemainSlotOnZero TargetToConsume)
                (Utilities|Map|Add (Variables|Default|GetDict_ItemContainer) TargetToConsume (Math|Integer|Clamp(Integer) _returnvalue_2 0 999) :!label _label)
                (Default|CallEdItemUpdate TargetToConsume (.Value (Utilities|Map|Find (Variables|Default|GetDict_ItemContainer) TargetToConsume)))
                (elif (< _returnvalue_2 1)
                  (Utilities|Map|Remove _dict_itemcontainer TargetToConsume)
                  (Default|CallEdItemRemove TargetToConsume)
                  (else
                    (goto _label))))
              (else
                (return false)))
            (else
              (return false))))
        (:Is%20Not%20Valid
          (return false))))
    (:then_1
      (Variables|Default|SetLastestUsing 0))
    (:then_2
      (return true))))

(fn CheckifItemValid
  (params (TargetToCheck :type PMA%20Item%20Data%20Object%20Reference))
  (bind _dict_itemcontainer (Variables|Default|GetDict_ItemContainer))
  (bind (_value _returnvalue) (Utilities|Map|Find _dict_itemcontainer TargetToCheck))
  (Development|PrintString (Utilities|String|Append (Utilities|String|ToString(Boolean) _returnvalue) (Utilities|String|ToString(Integer) _value)))
  (return (and _returnvalue (> _value 0)) _value))

(fn UseItem
  (params (ItemToUse :type PMA%20Item%20Data%20Object%20Reference%20%28by%20ref%29))
  (bind _itemisvalid (CallFunction|CheckifItemValid ItemToUse))
  (if _itemisvalid
    (Development|PrintString "Isvalid")
    (Variables|Default|SetLastestUsing ItemToUse)
    (CallFunction|ConstructionItemScript (Variables|/Game/System/Item/PMA_ItemData.PMA_ItemData_C|GetSimpleAttachedScriptOnUse ItemToUse))))

(fn IsFunctionScriptCached
  (params (ObjectClass :type Object%20Class%20Reference))
  (bind _array_element (Utilities|Array|ForEachLoopwithBreak (Variables|Default|GetCacheUsingScript))
    (:LoopBody
      (if (Class|GameplayStatics|ObjectIsA _array_element ObjectClass)
        (return true _array_element)))
    (:Completed
      (return false 0))))