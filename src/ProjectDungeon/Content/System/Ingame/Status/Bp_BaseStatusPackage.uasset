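; Base status effect package for characters, holding setup data such as name, priority, duration, state tag, owner, raw values and buff flag.
; StartBlindingToUpdate caches the character and, unless duration is manual, binds to the GameState's global status interval event.
; Each interval decrements the countdown by 0.1 and calls the empty EachTickUpdate hook.
; At zero it unbinds and removes itself from the character, printing a debug string.
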(event `StartBlindingToUpdate`
  (params (Character :type "/Game/System/GameCharacter/Bp_BaseCharacter Object Reference"))
  (bind _output_get (set `self.CurrentCharacter` Character))
  (bind _asgs_ingame_game_state (`/Game/System/GameCharacter/Bp_BaseCharacter.GiveMeGameState` _output_get))
  (set `self.CountDuration` (`self.Duration`))
  (if (not (`self.MannualDuration`))
    (add `/Game/System/Ingame/GS_IngameGameState.Ed_StatusGlobalInterval` _asgs_ingame_game_state (delegate `CustomEvent`))))

(event `CustomEvent`
  (bind _currentcharacter (`self.CurrentCharacter`))
  (bind _output_get (set `self.CountDuration` (- (`self.CountDuration`) 0.1)))
  (`self.EachTickUpdate`)
  (if (<= _output_get 0.0)
    (remove `/Game/System/Ingame/GS_IngameGameState.Ed_StatusGlobalInterval` (stale `StartBlindingToUpdate` _asgs_ingame_game_state) (delegate `CustomEvent`))
    (`/Game/System/GameCharacter/Bp_BaseCharacter.RemoveStatus` _currentcharacter self)
    (`KismetSystemLibrary.PrintString` _currentcharacter "TryRemoveStatus")))

(event `EachTickUpdate`)

(fn `GetValuesAsTag`
  (params (StateTag :type "/Game/System/Ingame/Status/Struct_StatusTag Structure"))
  (returns (NewParam :type "Float (double-precision)"))
  (return (`self.RawValues`)))

(fn `SetupPackage`
  (params (StatusName :type String :default "Status?") (Description :type String) (Priority :type Integer :default 1) (Duration :type "Float (double-precision)" :default 1.0) (StateTag :type "/Game/System/Ingame/Status/Struct_StatusTag Structure") (SourceEvent :type "Actor Object Reference") (Owner :type "/Game/System/GameCharacter/Bp_BaseCharacter Object Reference") (RawValues :type "Float (double-precision)") (Variation :type Integer) (MannualDuration :type Boolean) (isBuff :type Boolean))
  (set `self.StatusName` StatusName)
  (set `self.Description` Description)
  (`|ExecutionSequence`
    (:`then_0`
      (set `self.Priority` Priority))
    (:`then_1`
      (set `self.Duration` Duration))
    (:`then_2`
      (set `self.StateTag` StateTag))
    (:`then_3`
      (set `self.SourceEvent` SourceEvent))
    (:`then_4`
      (set `self.Owner` Owner))
    (:`then_5`
      (set `self.RawValues` RawValues))
    (:`then_6`
      (set `self.Variation` Variation))
    (:`then_7`
      (set `self.MannualDuration` MannualDuration))
    (:`then_8`
      (set `self.isBuff` isBuff))
    (:`then_9`
      (return))))