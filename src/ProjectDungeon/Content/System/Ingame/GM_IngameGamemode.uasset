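; In-game GameMode for a dungeon game that spawns each player's chosen class: Tank, Attacker, Rogue or Cleric.
; SpawnDefaultPawnFor reads SelectedChar from the dungeon PlayerState and spawns the matching pawn at the start spot, with the default pawn as the fallback option.
; On each authoritative PostLogin it refreshes a cached array of all playable characters, exposed through GetAllPlayerCharacters.
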(event `self.ReceiveBeginPlay`
  (`parent.ReceiveBeginPlay`))

(event `self.K2_PostLogin`
  (params (NewPlayer :type "PlayerController Object Reference"))
  (`parent.K2_PostLogin` NewPlayer)
  (`KismetSystemLibrary.PrintString` (`KismetStringLibrary.Concat_StrStr` "LoggedIn" (`KismetSystemLibrary.GetDisplayName` NewPlayer)))
  (`/Engine/EditorBlueprintResources/ActorMacros.Switch Has Authority`
    (:`Authority`
      (bind _outactors (`GameplayStatics.GetAllActorsOfClass` "/Game/System/GameCharacter/Bp_BasePlayableCharacter.Bp_BasePlayableCharacter_C"))
      (set `self.AllPlayerCharacters` _outactors))))

(fn `GetAllPlayerCharacters`
  (returns (Characters :type "Array of /Game/System/GameCharacter/Bp_BasePlayableCharacter Object Reference"))
  (return (`self.AllPlayerCharacters`)))

(fn `SpawnDefaultPawnFor`
  (params (NewPlayer :type "Controller Object Reference") (StartSpot :type "Actor Object Reference"))
  (returns (ReturnValue :type "Pawn Object Reference"))
  (bind _asps_dungeon_player_state (cast `/Game/System/PS_DungeonPlayerState` (`Controller.PlayerState` NewPlayer)))
  (bind _selectedchar (`/Game/System/PS_DungeonPlayerState.SelectedChar` _asps_dungeon_player_state))
  (`KismetSystemLibrary.PrintString` (`KismetStringLibrary.Conv_IntToString` _selectedchar))
  (bind _returnvalue (`|SpawnActorFromClass` (select `int` _selectedchar :`0` (`self.DefaultPawnClass`) :`1` "/Game/System/GameCharacter/PlayerChar/PlayerC_Tank.PlayerC_Tank_C" :`2` "/Game/System/GameCharacter/PlayerChar/PlayerC_Attacker.PlayerC_Attacker_C" :`3` "/Game/System/GameCharacter/PlayerChar/PlayerC_Rogue.PlayerC_Rogue_C" :`4` "/Game/System/GameCharacter/PlayerChar/PlayerC_Cleric.PlayerC_Cleric_C" :!type "Actor Class Reference") (`self.GetTransform` StartSpot) "Undefined" "MultiplyWithRoot" NewPlayer null))
  (bind _aspawn (cast `Pawn` _returnvalue))
  (return _aspawn))

(fn `UserConstructionScript`)