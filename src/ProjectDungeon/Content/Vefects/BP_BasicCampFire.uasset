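; Campfire actor that periodically damages characters standing inside its sphere trigger.
; On the server, the first overlapping base character starts a looping half-second damage timer, which is cleared once the sphere holds no characters.
; Each tick sends damage to every overlapping character through the character interface, hitting those tagged Player twice as hard as others.
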(event `self.Sphere.OnComponentBeginOverlap`
  (params (OverlappedComponent :type "PrimitiveComponent Object Reference") (OtherActor :type "Actor Object Reference") (OtherComp :type "PrimitiveComponent Object Reference") (OtherBodyIndex :type Integer) (bFromSweep :type Boolean) (SweepResult :type "HitResult Structure (by ref)"))
  (`/Engine/EditorBlueprintResources/ActorMacros.Switch Has Authority`
    (:`Authority`
      (if (`KismetSystemLibrary.K2_IsValidTimerHandle` (`self.FireTimer`))
        _
        (elif (`GameplayStatics.ObjectIsA` OtherActor "/Game/System/GameCharacter/Bp_BaseCharacter.Bp_BaseCharacter_C")
          (`|ExecutionSequence`
            (:`then_1`
              (bind _returnvalue (`KismetSystemLibrary.K2_SetTimerDelegate` (delegate `DealDam,age`) 0.5 true))
              (set `self.FireTimer` _returnvalue))))))))

(event `self.Sphere.OnComponentEndOverlap`
  (params (OverlappedComponent :type "PrimitiveComponent Object Reference") (OtherActor :type "Actor Object Reference") (OtherComp :type "PrimitiveComponent Object Reference") (OtherBodyIndex :type Integer))
  (if (<= (`KismetArrayLibrary.Array_Length` (`PrimitiveComponent.GetOverlappingActors` (`self.Sphere`) "/Game/System/GameCharacter/Bp_BaseCharacter.Bp_BaseCharacter_C")) 0)
    (`KismetSystemLibrary.K2_ClearAndInvalidateTimerHandle` (`self.FireTimer`))))

(event `DealDam,age`
  (for _array_element (`PrimitiveComponent.GetOverlappingActors` (`self.Sphere`) "/Game/System/GameCharacter/Bp_BaseCharacter.Bp_BaseCharacter_C")
    (message `/Game/System/GameCharacter/Int_StatusPackage.InterfaceCharacterApplyDamage` _array_element (`KismetMathLibrary.SelectFloat` 10.0 5.0 (`self.ActorHasTag` _array_element "Player")) false self (0.0 0.0 0.0) 0.0)))

(fn `UserConstructionScript`)